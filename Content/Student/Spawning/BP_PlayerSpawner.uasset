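; Player spawner actor that supplies spawn locations and an associated GameMode value, with no active event logic of its own.
; GetSpawnPoints converts each SpawnPoints offset to world space by adding the actor's location, ignoring rotation and scale, and returns the resulting list.
; GetGameModeSpawner returns the GameMode value stored on the spawner.
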(fn `GetGameModeSpawner`
  (returns (GameMode :type "/Game/Student/Data/E_GameModes Enum"))
  (return (`self.GameMode`)))

(fn `GetSpawnPoints`
  (returns (SpawnPoints :type "Array of Vector Structure"))
  (locals (worldSpaceSpawnPoints :type "Array of Vector Structure"))
  (for _array_element (`self.SpawnPoints`)
    (`KismetArrayLibrary.Array_Add` (`local.worldSpaceSpawnPoints`) (+ (`self.K2_GetActorLocation`) _array_element)))
  (return (`local.worldSpaceSpawnPoints`)))

(fn `UserConstructionScript`)