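; Player controller that forwards input to its pawn and handles registration of local controllers with the game mode.
; Releasing RegisterController asks the game mode to register this controller, while Jump and Dash presses are sent as messages to the controlled pawn.
; SetID stores an assigned controller ID and marks it registered; GetControlloerID returns that ID and flag, or zero if unregistered, and prints the registration state.
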(event `InputAction|RegisterController`
  (params (Key :type "Key Structure"))
  (:`Released`
    (message `/Game/Student/Interfaces/BPI_MainMenu.RegisterController` (`GameplayStatics.GetGameMode`) self)))

(event `InputAction|Jump`
  (params (Key :type "Key Structure"))
  (:`Pressed`
    (message `/Game/Student/Gameplay/Character/Interfaces/BPI_CharacterActions.OnJump` (`self.K2_GetPawn`))))

(event `InputAction|Dash`
  (params (Key :type "Key Structure"))
  (:`Pressed`
    (message `/Game/Student/Gameplay/Character/Interfaces/BPI_CharacterActions.OnDash` (`self.K2_GetPawn`))))

(fn `GetControlloerID`
  (returns (isRegistered :type Boolean) (controllerID :type Integer))
  (`KismetSystemLibrary.PrintString` (`KismetStringLibrary.Concat_StrStr` "Controller is registered" (`KismetStringLibrary.Conv_BoolToString` (`self.isRegistered`))))
  (if (`self.isRegistered`)
    (return (`self.isRegistered`) (`self.controllerID`))
    (else
      (return false 0))))

(fn `SetID`
  (params (controllerID :type Integer))
  (set `self.controllerID` controllerID)
  (set `self.isRegistered` true))

(fn `UserConstructionScript`)