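; BP_Zombie is an AI zombie character with speed and health taken from AIData.
; A state setter switches Idle, Chase and Attack, notifying listeners and dispatching to Init functions, which are currently empty.
; GetNearestPlayer targets the closest living player from the game mode, choosing Chase or falling back to Idle.
; Damage reduces health, then either reports death to the attacker or starts a timed invulnerability window.
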(event `/Game/Student/Gameplay/Character/Interfaces/BPI_Zombie.UpdateZombieState`
  (params (NewState :type "/Game/Student/Gameplay/ZombieSurvival/AI/Data/E_ZombieStates Enum" :default "NewEnumerator0"))
  (`self.SetNewState` NewState))

(event `/Game/Student/Gameplay/Character/Interfaces/BPI_Hurtable.DamageActor`
  (params (InterfaceActor :type "Actor Object Reference") (dmg :type "Float (single-precision)"))
  (if (`self.CanBehurt`)
    (bind _output_get (set `self.currentHealth` (- (`self.currentHealth`) dmg)))
    (if (<= _output_get 0.0)
      (message `/Game/Student/Gameplay/Character/Interfaces/BPI_Hurtable.DamageActorDied` InterfaceActor self)
      (else
        (set `self.CanBehurt` false)
        (`self.StartHurtTime`)))))

(fn `EvaluateNewState`
  (`self.SwitchStates`
    (:`Idle`
      (`self.InitIdle`))
    (:`Chase`
      (`self.InitChase`))
    (:`Attack`
      (`self.InitAttack`))))

(fn `Get Alive Players`
  (returns (PlayersAlive :type "Array of /Game/Student/Gameplay/Character/BP_BaseTeamCharacter Object Reference"))
  (locals (alivePlayers :type "Array of /Game/Student/Gameplay/Character/BP_BaseTeamCharacter Object Reference"))
  (bind _players (message `/Game/Student/Interfaces/BPI_GamemodeData.GetPlayers` (`GameplayStatics.GetGameMode`)))
  (for _array_element _players
    (bind _isalive (`/Game/Student/Gameplay/Character/BP_BaseTeamCharacter.GetIsAlive` _array_element))
    (if _isalive
      (`KismetArrayLibrary.Array_Add` (`local.alivePlayers`) _array_element)))
  (return (`local.alivePlayers`)))

(fn `GetNearestPlayer`
  (locals (CurrShortestDistance :type "Float (double-precision)") (playerAlive :type "Array of /Game/Student/Gameplay/Character/BP_BaseTeamCharacter Object Reference") (shortestIndex :type Integer))
  (bind _output (`|GetArrayItem` (`local.playerAlive`) (`local.shortestIndex`)))
  (bind _playersalive (`self.Get Alive Players`))
  ;[1 1 1] Assume first element is the shortest distance
  (bind _output_get (set `local.playerAlive` _playersalive))
  (set `local.CurrShortestDistance` (`KismetMathLibrary.Vector_Distance` (`self.K2_GetActorLocation` (`|GetArrayItem` _output_get)) (`self.K2_GetActorLocation`)))
  (for (_array_element _array_index) (`local.playerAlive`)
    (bind _returnvalue (`KismetMathLibrary.Vector_Distance` (`self.K2_GetActorLocation` _array_element) (`self.K2_GetActorLocation`)))
    (if (<= _returnvalue (`local.CurrShortestDistance`))
      ;[1 1 1] Set the newest shortest distance and store index to element
      (set `local.CurrShortestDistance` _returnvalue)
      (set `local.shortestIndex` _array_index)))
  ;[1 1 1] Check if value is valid
  (`/Engine/EditorBlueprintResources/StandardMacros.IsValid` _output
    (:`Is Valid`
      ;[1 1 1] If it is chase target
      (set `self.currentTarget` _output)
      (`self.SetNewState` "NewEnumerator1"))
    (:`Is Not Valid`
      ;[1 1 1] Else be idle
      (`self.SetNewState` "NewEnumerator0"))))

(fn `GetZombieAIData`
  (returns (GetZombieData :type "/Game/Student/Gameplay/ZombieSurvival/AI/Data/S_ZombieData Structure") (GetCurrentTarget :type "Actor Object Reference"))
  (return (`self.AIData`) null))

(fn `InitAttack`)

(fn `InitChase`)

(fn `InitIdle`)

(fn `ResetHurt`
  (set `self.CanBehurt` true))

(fn `SetNewState`
  (params (NewState :type "/Game/Student/Gameplay/ZombieSurvival/AI/Data/E_ZombieStates Enum" :default "NewEnumerator0"))
  (bind _output_get (set `self.currentState` NewState))
  (`self.OnStateChange` _output_get)
  (`self.EvaluateNewState`))

(fn `SetUp`
  (bind (_aidata_attackrange _aidata_attackspeed _aidata_movememtspeed _aidata_mindamage _aidata_maxdamage _aidata_maxhealth) (break `/Game/Student/Gameplay/ZombieSurvival/AI/Data/S_ZombieData` (`self.AIData`)))
  (set `CharacterMovementComponent.MaxWalkSpeed` _aidata_movememtspeed (`self.CharacterMovement`))
  (set `self.currentHealth` _aidata_maxhealth))

(fn `StartHurtTime`
  (bind _returnvalue (`KismetSystemLibrary.K2_SetTimer` null "ResetHurt" (`self.HurtTime`)))
  (set `self.HurtTimerHandle` _returnvalue))

(fn `UserConstructionScript`)