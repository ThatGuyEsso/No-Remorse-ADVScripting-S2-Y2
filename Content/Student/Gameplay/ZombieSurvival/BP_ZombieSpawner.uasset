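; BP_ZombieSpawner is a spawner actor that creates AI-controlled zombies at random intervals for the zombie survival mode.
; Game mode events start spawning when the game runs, pause it at enemy capacity and resume it when space frees up.
; A one-shot timer re-arms itself after each spawn.
; SpawnZombie spawns a zombie and its AI controller, possesses and initializes it, notifies the game mode and assigns its team.
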(event `/Game/Student/Interfaces/BPI_Init.InitActor`
  ;[1 1 1] Init spawning
  (bind _zombiegamemode (message `/Game/Student/Interfaces/BPI_ZombieSurvival.GetZombieGameModeRef` (`GameplayStatics.GetGameMode`)))
  (add `/Game/Student/GameModes/GM_ZombieSurvial.OnEnemyCapacityReached` _zombiegamemode (delegate `OnCapacityReached`))
  (add `/Game/Student/GameModes/GM_ZombieSurvial.OnNotAtEnemyCapacity` _zombiegamemode (delegate `OnAvailableCapacity`))
  (add `/Game/Student/GameModes/GM_ZombieSurvial.OnNewState` _zombiegamemode (delegate `OnNewState`)))

(event `OnNewState`
  (params (newState :type "/Game/Student/Data/E_GameStates Enum" :default "NewEnumerator0"))
  ;[1 1 1] Init spawning
  (switch `/Game/Student/Data/E_GameStates` newState
    (:`NewEnumerator5`
      (set `self.CanSpawn` true)
      (`self.OnResetSpawnTimer`))))

(event `OnAvailableCapacity`
  ;[1 1 1] Init spawning
  ;;[0.09339 1 0.2877] On no longer at capacity
  (set `self.CanSpawn` true)
  (`self.OnResetSpawnTimer`))

(event `OnCapacityReached`
  ;[1 1 1] Init spawning
  ;;[1 0.3407 0.4466] On Capacity Reached
  (set `self.CanSpawn` false))

(event `OnResetSpawnTimer`
  ;[1 1 1] On Reset timer
  (bind _returnvalue (`KismetSystemLibrary.K2_SetTimerDelegate` (delegate `OnSpawnZombie`) (`KismetMathLibrary.RandomFloatInRange` (`self.minSpawnTime`) (`self.maxSpawn`))))
  (set `self.SpawnTimer` _returnvalue))

(event `OnSpawnZombie`
  ;[1 1 1] On Spawn Zombie
  (if (`self.CanSpawn`)
    (`self.SpawnZombie`)
    (`self.OnResetSpawnTimer`)))

(fn `GetPlayers`
  (returns (Players :type "Array of /Game/Student/Gameplay/Character/BP_BaseTeamCharacter Object Reference"))
  (return))

(fn `GetZombieAIData`
  (returns (GetZombieData :type "/Game/Student/Gameplay/ZombieSurvival/AI/Data/S_ZombieData Structure") (GetCurrentTarget :type "Actor Object Reference"))
  (return (struct) null))

(fn `GetZombieGameModeRef`
  (returns (ZombieGameMode :type "/Game/Student/GameModes/GM_ZombieSurvial Object Reference"))
  (return null))

(fn `IsAtZombieCapacity`
  (returns (IsAtCapacity :type Boolean))
  (return false))

(fn `SpawnZombie`
  (locals (currentController :type "/Game/Student/Controllers/AIC_ZombieController Object Reference") (CurrentZombie :type "/Game/Student/Gameplay/Character/BP_Zombie Object Reference"))
  (bind _currentzombie (`local.CurrentZombie`))
  (bind _returnvalue (`|SpawnActorFromClass` "/Game/Student/Controllers/AIC_ZombieController.AIC_ZombieController_C" (`KismetMathLibrary.MakeTransform` (0.0 0.0 0.0)) "Undefined" "OverrideRootScale" null null))
  (set `local.currentController` _returnvalue)
  (bind _returnvalue_2 (`|SpawnActorFromClass` "/Game/Student/Gameplay/Character/BP_Zombie.BP_Zombie_C" (`KismetMathLibrary.MakeTransform` (`SceneComponent.K2_GetComponentLocation` (`self.SpawnPoint`))) "Undefined" "OverrideRootScale" null null))
  (bind _output_get (set `local.CurrentZombie` _returnvalue_2))
  (`Controller.Possess` (`local.currentController`) _output_get)
  (`/Game/Student/Gameplay/Character/BP_Zombie.SetUp` (`local.CurrentZombie`))
  (`/Game/Student/Controllers/AIC_ZombieController.InitController` (`local.currentController`))
  (message `/Game/Student/Interfaces/BPI_ZombieSurvival.NewZombieSpawned` (`GameplayStatics.GetGameMode`))
  (message `/Game/Student/Interfaces/BPI_TeamData.AssignTeam` _currentzombie "NewEnumerator3")
  (`/Game/Student/Gameplay/Character/BP_Zombie.GetNearestPlayer` _currentzombie))

(fn `UserConstructionScript`)