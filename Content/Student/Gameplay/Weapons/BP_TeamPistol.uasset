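; BP_TeamPistol is a team-aware pistol weapon that shoots projectiles on behalf of its owning Character.
; Its Fire function spawns a BP_TeamProjectile at the Character's fire point, always spawning regardless of collision.
; The projectile receives the Character's team, armour colour and a fixed damage, with the Character as owner and instigator.
; The event graph holds only disabled stub events.
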(fn `Fire`
  (bind _character (`self.Character`))
  (bind (_newparam_location _newparam_rotation) (`KismetMathLibrary.BreakTransform` (`/Game/Framework_Blueprints/Characters/BP_BaseCharacter.GetFirePoint` (`self.Character`))))
  (bind _team (message `/Game/Student/Interfaces/BPI_TeamData.GetTeam` _character))
  (`|SpawnActorFromClass` "/Game/Student/Gameplay/Weapons/BP_TeamProjectile.BP_TeamProjectile_C" (`KismetMathLibrary.MakeTransform` _newparam_location _newparam_rotation (1.0 1.0 1.0)) "AlwaysSpawn" "OverrideRootScale" _character _team (`/Game/Framework_Blueprints/Characters/BP_BaseCharacter.ArmourColour` _character) 20.0 _character))

(fn `UserConstructionScript`
  (`parent.UserConstructionScript`))