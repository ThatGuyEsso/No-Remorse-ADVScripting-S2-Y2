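; Manager for the score level that dresses the winner and loser podiums with player results from the GameInstance.
; SetUpWinner and SetUpLoser each read the player data message, pass player identity, colour and score to their mannequin, and tint that podium's light to match.
; The winner always takes the message's PlayerOne entry and the loser PlayerTwo, with no score comparison here.
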(event `SetUpWinner`
  (bind _playerone (message `/Game/Student/Blueprint/Interfaces/BPI_GameData.GetPlayerData` (`GameplayStatics.GetGameInstance`)))
  (`/Game/Student/Blueprint/Props/BP_Playermannequin.OnSetUpMannequin` (`self.WinnerMannequin`) (`.IsPlayerOne_8_4520C6C14351485178668FB62F17DFA7` (break `/Game/Student/Blueprint/Data/S_PlayerData` _playerone)) (`.PlayerColour_5_F8D8D5A242847EF448AAE992D248BB5D` (break `/Game/Student/Blueprint/Data/S_PlayerData` _playerone)) (break `/Game/Student/Blueprint/Data/S_PlayerData` _playerone))
  (`/Game/Student/Blueprint/Props/BP_WallLight.SetWallColour` (`self.WinnerPodiumLight`) (`KismetMathLibrary.Conv_ColorToLinearColor` (`.PlayerColour_5_F8D8D5A242847EF448AAE992D248BB5D` (break `/Game/Student/Blueprint/Data/S_PlayerData` _playerone)))))

(event `SetUpLoser`
  (bind (_playerone _playertwo) (message `/Game/Student/Blueprint/Interfaces/BPI_GameData.GetPlayerData` (`GameplayStatics.GetGameInstance`)))
  (`/Game/Student/Blueprint/Props/BP_Playermannequin.OnSetUpMannequin` (`self.LoserManneQuin`) (`.IsPlayerOne_8_4520C6C14351485178668FB62F17DFA7` (break `/Game/Student/Blueprint/Data/S_PlayerData` _playertwo)) (`.PlayerColour_5_F8D8D5A242847EF448AAE992D248BB5D` (break `/Game/Student/Blueprint/Data/S_PlayerData` _playertwo)) (break `/Game/Student/Blueprint/Data/S_PlayerData` _playertwo))
  (`/Game/Student/Blueprint/Props/BP_WallLight.SetWallColour` (`self.LoserPodiumLight`) (`KismetMathLibrary.Conv_ColorToLinearColor` (`.PlayerColour_5_F8D8D5A242847EF448AAE992D248BB5D` (break `/Game/Student/Blueprint/Data/S_PlayerData` _playertwo)))))

(fn `UserConstructionScript`)