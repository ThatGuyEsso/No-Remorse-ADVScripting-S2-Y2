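; Wave manager for a zombie survival mode that runs timed waves with cooldowns from the "Survival" data table row.
; When the game mode enters Game Running, it initialises the spawners and starts the first wave.
; Each wave sets the game mode's zombie cap and spawners' rate bounds, while named timers chain waves until survival ends.
; OnWaveStart/End events drive a state that a looping timer uses to refresh the countdown widget.
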(event `/Game/Student/Blueprint/Interfaces/BPI_Init.InitActor`
  (`self.SetUpWaveData` "Survival")
  (set `self.CurrentWave` 0)
  (bind _zombiegamemode (message `/Game/Student/Blueprint/Interfaces/BPI_ZombieSurvival.GetZombieGameModeRef` (`GameplayStatics.GetGameMode`)))
  (add `/Game/Student/Blueprint/GameModes/GM_ZombieSurvial.OnNewState` _zombiegamemode (delegate `On Newstae`))
  (add `self.OnWaveStart` (delegate `WaveStart`))
  (add `self.OnWaveEnd` (delegate `WaveEnd`))
  (add `self.OnZombieSurvivalEnded` (delegate `OnGameEnded`)))

(event `WaveStart`
  (`self.SetUpTime`)
  (set `self.WaveState` "NewEnumerator0")
  (`/Game/Student/Blueprint/Widgets/BPW_WaveTimer.Update Wave Label` (`self.WaveTimeDisplay`) (`self.CurrentWave`))
  (`KismetSystemLibrary.K2_PauseTimerHandle` (`self.CoolDownTimer`)))

(event `WaveEnd`
  (`self.SetUpTime`)
  (set `self.WaveState` "NewEnumerator1")
  (`KismetSystemLibrary.K2_PauseTimerHandle` (`self.CurrentWaveTimer`)))

(event `OnGameEnded`
  (set `self.WaveState` "NewEnumerator2"))

(event `On Newstae`
  (params (newState :type "/Game/Student/Blueprint/Data/E_GameStates Enum" :default "NewEnumerator0"))
  (switch `/Game/Student/Blueprint/Data/E_GameStates` newState
    (:`NewEnumerator5`
      (for _array_element (`self.spawners`)
        (set `/Game/Student/Blueprint/Gameplay/ZombieSurvival/BP_ZombieSpawner.WaveManager` self _array_element)
        (`/Game/Student/Blueprint/Gameplay/ZombieSurvival/BP_ZombieSpawner.InitActor` _array_element))
      (`self.StartNextWave`)
      (bind _returnvalue (`KismetSystemLibrary.K2_SetTimerDelegate` (delegate `OnUpdateTimer`) 0.2 true))
      (set `self.DisplayUpdateTimer` _returnvalue))))

(event `OnUpdateTimer`
  (switch `/Game/Student/Blueprint/Spawning/E_WaveState` (`self.WaveState`)
    (:`NewEnumerator0`
      (`/Game/Student/Blueprint/Widgets/BPW_WaveTimer.UpdateDisplay` (`self.WaveTimeDisplay`) (`KismetMathLibrary.FCeil` (- (`self.waveTime`) (`KismetSystemLibrary.K2_GetTimerElapsedTimeHandle` (`self.CurrentWaveTimer`))))))
    (:`NewEnumerator1`
      (`/Game/Student/Blueprint/Widgets/BPW_WaveTimer.UpdateDisplay` (`self.WaveTimeDisplay`) (`KismetMathLibrary.FCeil` (- (`self.CoolDownTime`) (`KismetSystemLibrary.K2_GetTimerElapsedTimeHandle` (`self.CoolDownTimer`))))))
    (:`NewEnumerator2`
      (`KismetSystemLibrary.K2_PauseTimerHandle` (`self.DisplayUpdateTimer`)))))

(fn `EndWave`
  (bind _waves_allwaves (break `/Game/Student/Blueprint/Spawning/S_Waves` (`self.Waves`)))
  (`self.OnWaveEnd`)
  (bind _result (`/Engine/EditorBlueprintResources/StandardMacros.IncrementInt` (`self.CurrentWave`))
    (:`  `
      (if (< _result (`KismetArrayLibrary.Array_Length` _waves_allwaves))
        (bind _returnvalue (`KismetSystemLibrary.K2_SetTimer` null "StartNextWave" (`self.CoolDownTime`)))
        (set `self.CoolDownTimer` _returnvalue)
        (`/Game/Student/Blueprint/Widgets/BPW_WaveTimer.DisplayCooldown` (`self.WaveTimeDisplay`))
        (else
          (`self.OnZombieSurvivalEnded`))))))

(fn `GetSetUpData`
  (returns (Data :type "/Game/Student/Blueprint/Data/S_SetUpData Structure"))
  (return))

(fn `GetZombieGameModeRef`
  (returns (ZombieGameMode :type "/Game/Student/Blueprint/GameModes/GM_ZombieSurvial Object Reference"))
  (return null))

(fn `IsAtZombieCapacity`
  (returns (IsAtCapacity :type Boolean))
  (return false))

(fn `SetUpTime`
  (`/Engine/EditorBlueprintResources/StandardMacros.IsValid` (`self.WaveTimeDisplay`)
    (:`Is Valid`
      _)
    (:`Is Not Valid`
      (bind _returnvalue (`|CreateWidget` "/Game/Student/Blueprint/Widgets/BPW_WaveTimer.BPW_WaveTimer_C"))
      (bind _output_get (set `self.WaveTimeDisplay` _returnvalue))
      (`UserWidget.AddToViewport` (`self.WaveTimeDisplay`) 0)
      (`UserWidget.AddToViewport` _output_get 0)))
  (`/Game/Student/Blueprint/Widgets/BPW_WaveTimer.UpdateDisplay` (`self.WaveTimeDisplay`) (`KismetMathLibrary.FCeil` (`KismetSystemLibrary.K2_GetTimerElapsedTimeHandle` (`self.CurrentWaveTimer`)))))

(fn `SetUpWaveData`
  (params (RowName :type Name))
  (bind _returnvalue (`|GetDataTableRow` (`self.WavesData`) RowName)
    (:`then`
      (set `self.Waves` _returnvalue))))

(fn `StartNextWave`
  (bind _waves_allwaves (break `/Game/Student/Blueprint/Spawning/S_Waves` (`self.Waves`)))
  (bind (_maxzombies _wavetime _minspawnrate _maxspawnrate) (break `/Game/Student/Blueprint/Spawning/S_WaveData` (`|GetArrayItem` _waves_allwaves (`self.CurrentWave`))))
  (message `/Game/Student/Blueprint/Interfaces/BPI_ZombieSurvival.SetMaxZombies` (`GameplayStatics.GetGameMode`) _maxzombies)
  (set `self.waveTime` _wavetime)
  (if (> (`KismetArrayLibrary.Array_Length` (`self.spawners`)) 0)
    (for _array_element (`self.spawners`)
      (`/Game/Student/Blueprint/Gameplay/ZombieSurvival/BP_ZombieSpawner.SetSpawnRateBounds` _array_element _minspawnrate _maxspawnrate))
    (bind _returnvalue (`KismetSystemLibrary.K2_SetTimer` null "EndWave" (`self.waveTime`)))
    (set `self.CurrentWaveTimer` _returnvalue)
    (`self.OnWaveStart`)
    (message `/Game/Student/Blueprint/Interfaces/BPI_ZombieSurvival.RefreshZombieLimit` (`GameplayStatics.GetGameMode`))))

(fn `UserConstructionScript`)