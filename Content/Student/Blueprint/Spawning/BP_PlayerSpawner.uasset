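; BP_PlayerSpawner is an actor that respawns players after SpawnDelay by moving them to a random spawn point.
; RespawnPlayer uses two timer slots: EarliestRespawn normally, LatestRespawn while the first timer runs, so further overlapping requests overwrite LatestRespawn.
; When a timer fires, it relocates that player and calls RespawnMessage.
; SpawnPoints are offsets from the actor's location, and the random pick never selects the last one.
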(event `RespawnPlayer`
  (params (player :type "Actor Object Reference"))
  (if (`KismetSystemLibrary.K2_IsTimerActiveHandle` (`self.PrimSpawnLoop`))
    (`KismetSystemLibrary.K2_SetTimerDelegate` (delegate `LateRespawn`) (`self.SpawnDelay`))
    (set `self.latestRespawn` player)
    (else
      (bind _returnvalue (`KismetSystemLibrary.K2_SetTimerDelegate` (delegate `OnRespawnedEarlyDeath`) (`self.SpawnDelay`)))
      (set `self.PrimSpawnLoop` _returnvalue)
      (set `self.earliestRespawn` player))))

(event `LateRespawn`
  (`self.K2_SetActorLocation` (`self.latestRespawn`) (+ (`|GetArrayItem` (`self.SpawnPoints`) (`KismetMathLibrary.RandomInteger` (`KismetArrayLibrary.Array_LastIndex` (`self.SpawnPoints`)))) (`self.K2_GetActorLocation`)) false false)
  (message `/Game/Student/Blueprint/Gameplay/Characters/Interfaces/BPI_CharacterActions.Respawn` (`self.latestRespawn`)))

(event `OnRespawnedEarlyDeath`
  (`self.K2_SetActorLocation` (`self.earliestRespawn`) (+ (`|GetArrayItem` (`self.SpawnPoints`) (`KismetMathLibrary.RandomInteger` (`KismetArrayLibrary.Array_LastIndex` (`self.SpawnPoints`)))) (`self.K2_GetActorLocation`)) false false)
  (message `/Game/Student/Blueprint/Gameplay/Characters/Interfaces/BPI_CharacterActions.Respawn` (`self.earliestRespawn`)))

(fn `GetGameModeSpawner`
  (returns (GameMode :type "/Game/Student/Blueprint/Data/E_GameModes Enum"))
  (return (`self.GameMode`)))

(fn `GetSpawnPoints`
  (returns (SpawnPoints :type "Array of Vector Structure"))
  (locals (worldSpaceSpawnPoints :type "Array of Vector Structure"))
  (for _array_element (`self.SpawnPoints`)
    (`KismetArrayLibrary.Array_Add` (`local.worldSpaceSpawnPoints`) (+ (`self.K2_GetActorLocation`) _array_element)))
  (return (`local.worldSpaceSpawnPoints`)))

(fn `UserConstructionScript`)