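; Game mode for the score scene between minigames, showing the two players' standings and leading on to the next game or main menu.
; An event-driven state machine recreates local players on the scene camera, finds BP_ScoreLevelManager, then evaluates scores from game instance data.
; Results feed the level manager and score widget, while games remaining decide the next mode.
; On Next, it opens Arena with that mode's option, or MainMenu once games run out.
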(event `self.ReceiveBeginPlay`
  (add `self.NewState` (delegate `OnNewState`))
  (`self.NewState` "NewEnumerator0"))

(event `OnNewState` :!signature `self.NewState`
  (params (newState :type "/Game/Student/Blueprint/Data/E_ScoreScreenStates Enum" :default "NewEnumerator0"))
  (switch `/Game/Student/Blueprint/Data/E_ScoreScreenStates` newState
    (:`NewEnumerator0`
      (`self.SetUpController`))
    (:`NewEnumerator1`
      (`self.SetUpManager`))
    (:`NewEnumerator4`
      (`self.EvaluateWinners`)
      (`self.EvaluateNextGameMode`))
    (:`NewEnumerator2`
      (`self.InitNextGameMode`))))

(event `self.K2_PostLogin`
  (params (NewPlayer :type "PlayerController Object Reference"))
  ;[1 1 1] Controller Log in
  (bind _aspc_player_character (cast `/Game/Student/Blueprint/Controllers/PC_PlayerCharacter` NewPlayer))
  (set `PlayerController.bShowMouseCursor` true _aspc_player_character)
  (`KismetArrayLibrary.Array_Add` (`self.PlayerControllers`) _aspc_player_character))

(event `self.K2_OnLogout`
  (params (ExitingController :type "Controller Object Reference"))
  ;[1 1 1] Controller Log in
  (bind _aspc_player_character (cast `/Game/Student/Blueprint/Controllers/PC_PlayerCharacter` ExitingController))
  (`KismetArrayLibrary.Array_RemoveItem` (`self.PlayerControllers`) _aspc_player_character))

(event `self.OnQuit`
  (`KismetSystemLibrary.QuitGame` null "Quit"))

(event `self.OnNext`
  (`self.NewState` "NewEnumerator2"))

(event `self.OnMainMenu`
  (for _array_element (`self.PlayerControllers`)
    (`GameplayStatics.RemovePlayer` _array_element true))
  (`GameplayStatics.OpenLevel` "MainMenu"))

(fn `EvaluateNextGameMode`
  (locals (GamesLeft :type Integer :default 0) (index :type Integer))
  (bind _returnvalue (`GameplayStatics.GetGameInstance`))
  (bind _gamesleft (message `/Game/Student/Blueprint/Interfaces/BPI_GameData.GetNumberOfGamesLeft` _returnvalue))
  (bind _output_get (set `local.GamesLeft` _gamesleft))
  (if (> _output_get 0)
    (bind _totalgames (message `/Game/Student/Blueprint/Interfaces/BPI_GameData.GetGamesTotal` _returnvalue))
    (bind _output_get_2 (set `local.index` (- _totalgames (`local.GamesLeft`))))
    (bind _gamemode (message `/Game/Student/Blueprint/Interfaces/BPI_GameData.GetNextGameMode` (`GameplayStatics.GetGameInstance`) _output_get_2))
    (set `self.nextGameMode` _gamemode)
    (else
      (set `self.GameEnded` true)
      (`/Game/Student/Blueprint/Widgets/BPW_ScoreScreen.UpdatePointState` (`self.ScoreDisplay`) (`self.isTie`)))))

(fn `EvaluateWinners`
  (set `self.States` "NewEnumerator4")
  (bind (_playerone _playertwo) (message `/Game/Student/Blueprint/Interfaces/BPI_GameData.GetPlayerData` (`GameplayStatics.GetGameInstance`)))
  (bind _output_get (set `self.isTie` (== (break `/Game/Student/Blueprint/Data/S_PlayerData` _playerone) (break `/Game/Student/Blueprint/Data/S_PlayerData` _playertwo))))
  (if _output_get
    (bind _returnvalue (`|CreateWidget` "/Game/Student/Blueprint/Widgets/BPW_ScoreScreen.BPW_ScoreScreen_C"))
    (bind _output_get_2 (set `self.ScoreDisplay` _returnvalue))
    (`/Game/Student/Blueprint/Widgets/BPW_ScoreScreen.UpdatePointState` _output_get_2 true)
    (`UserWidget.AddToViewport` _output_get_2 0)
    (bind (_playerone_2 _playertwo_2) (message `/Game/Student/Blueprint/Interfaces/BPI_GameData.GetPlayerData` (`GameplayStatics.GetGameInstance`) :!label _label))
    (`/Game/Student/Blueprint/GameManagers/BP_ScoreLevelManager.SetUpWinner` (`self.ScoreDisplayManager`) true (`.PlayerColour_5_F8D8D5A242847EF448AAE992D248BB5D` (break `/Game/Student/Blueprint/Data/S_PlayerData` _playerone_2)) (break `/Game/Student/Blueprint/Data/S_PlayerData` _playerone_2))
    (`/Game/Student/Blueprint/GameManagers/BP_ScoreLevelManager.SetUpLoser` (`self.ScoreDisplayManager`) false (`.PlayerColour_5_F8D8D5A242847EF448AAE992D248BB5D` (break `/Game/Student/Blueprint/Data/S_PlayerData` _playertwo_2)) (break `/Game/Student/Blueprint/Data/S_PlayerData` _playertwo_2))
    (elif (> (break `/Game/Student/Blueprint/Data/S_PlayerData` _playerone) (break `/Game/Student/Blueprint/Data/S_PlayerData` _playertwo))
      (bind _returnvalue_2 (`|CreateWidget` "/Game/Student/Blueprint/Widgets/BPW_ScoreScreen.BPW_ScoreScreen_C"))
      (bind _output_get_3 (set `self.ScoreDisplay` _returnvalue_2))
      (`/Game/Student/Blueprint/Widgets/BPW_ScoreScreen.DisplayPointLeader` _output_get_3 true (`KismetMathLibrary.Conv_ColorToLinearColor` (`.PlayerColour_5_F8D8D5A242847EF448AAE992D248BB5D` (break `/Game/Student/Blueprint/Data/S_PlayerData` _playerone))))
      (`/Game/Student/Blueprint/Widgets/BPW_ScoreScreen.DisplayCurrentPointLeader` _output_get_3)
      (`UserWidget.AddToViewport` _output_get_3 0)
      (goto _label)
      (else
        (bind (_playerone_3 _playertwo_3) (message `/Game/Student/Blueprint/Interfaces/BPI_GameData.GetPlayerData` (`GameplayStatics.GetGameInstance`)))
        (`/Game/Student/Blueprint/GameManagers/BP_ScoreLevelManager.SetUpWinner` (`self.ScoreDisplayManager`) false (`.PlayerColour_5_F8D8D5A242847EF448AAE992D248BB5D` (break `/Game/Student/Blueprint/Data/S_PlayerData` _playertwo_3)) (break `/Game/Student/Blueprint/Data/S_PlayerData` _playertwo_3))
        (`/Game/Student/Blueprint/GameManagers/BP_ScoreLevelManager.SetUpLoser` (`self.ScoreDisplayManager`) true (`.PlayerColour_5_F8D8D5A242847EF448AAE992D248BB5D` (break `/Game/Student/Blueprint/Data/S_PlayerData` _playerone_3)) (break `/Game/Student/Blueprint/Data/S_PlayerData` _playerone_3))
        (bind _returnvalue_3 (`|CreateWidget` "/Game/Student/Blueprint/Widgets/BPW_ScoreScreen.BPW_ScoreScreen_C"))
        (bind _output_get_4 (set `self.ScoreDisplay` _returnvalue_3))
        (`/Game/Student/Blueprint/Widgets/BPW_ScoreScreen.DisplayCurrentPointLeader` _output_get_4)
        (`/Game/Student/Blueprint/Widgets/BPW_ScoreScreen.DisplayPointLeader` _output_get_4 false (`KismetMathLibrary.Conv_ColorToLinearColor` (`.PlayerColour_5_F8D8D5A242847EF448AAE992D248BB5D` (break `/Game/Student/Blueprint/Data/S_PlayerData` _playertwo_3))))
        (`UserWidget.AddToViewport` _output_get_4 0)))))

(fn `InitNextGameMode`
  (set `self.States` "NewEnumerator2")
  (if (`self.GameEnded`)
    (`self.OnMainMenu`)
    (else
      (for _array_element (`self.PlayerControllers`)
        (`GameplayStatics.RemovePlayer` _array_element true))
      (switch `/Game/Student/Blueprint/Data/E_GameModes` (`self.nextGameMode`)
        (:`NewEnumerator0`
          (`GameplayStatics.OpenLevel` "Arena" true "game=ZS"))
        (:`NewEnumerator1`
          (`GameplayStatics.OpenLevel` "Arena" true "game=BR"))
        (:`NewEnumerator2`
          (`GameplayStatics.OpenLevel` "Arena" true "game=KTH"))))))

(fn `SetUpController`
  (set `self.States` "NewEnumerator0")
  (bind _data (message `/Game/Student/Blueprint/Interfaces/BPI_GameData.GetSetUpData` (`GameplayStatics.GetGameInstance`)))
  (`GameplayStatics.RemovePlayer` (`GameplayStatics.GetPlayerController` 0) true)
  (for _ (range (break `/Game/Student/Blueprint/Data/S_SetUpData` _data))
    (bind _returnvalue (`GameplayStatics.CreatePlayer` -1))
    (bind _returnvalue_2 (`GameplayStatics.GetActorOfClass` "/Script/Engine.CameraActor"))
    (`PlayerController.SetViewTargetWithBlend` _returnvalue _returnvalue_2 0.0 "VTBlend_Linear" 0.0 false)
    (`self.NewState` "NewEnumerator1")))

(fn `SetUpManager`
  (set `self.States` "NewEnumerator1")
  (bind _returnvalue (`GameplayStatics.GetActorOfClass` "/Game/Student/Blueprint/GameManagers/BP_ScoreLevelManager.BP_ScoreLevelManager_C"))
  (set `self.ScoreDisplayManager` _returnvalue)
  (`self.NewState` "NewEnumerator4"))

(fn `UserConstructionScript`)