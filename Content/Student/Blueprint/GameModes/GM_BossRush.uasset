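; Game mode for Boss Rush, where players share a multiplayer camera in an arena with a boss.
; An OnNewState dispatcher chains setup states: controllers, random spawn points (repeats possible), possessed characters on one team, camera, scores, then game start.
; InitGame initialises the placed boss and a random weapon spawner, which it finds by the King of the Hill tag.
; Ending shows the game-over widget, stores player data, decrements games left and opens the score screen.
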(event `self.ReceiveBeginPlay`
  (add `self.OnNewState` (delegate `self.OnGameStateChange`))
  (`self.OnNewState` "NewEnumerator0"))

(event `self.OnGameStateChange`
  (params (newState :type "/Game/Student/Blueprint/Data/E_GameStates Enum" :default "NewEnumerator0"))
  (switch `/Game/Student/Blueprint/Data/E_GameStates` newState
    (:`NewEnumerator0`
      (`self.Init`))
    (:`NewEnumerator3`
      (`self.OnNewState` "NewEnumerator1"))
    (:`NewEnumerator1`
      (`self.SetUpSpawnPoints`))
    (:`NewEnumerator2`
      (`self.InitCharacters`))
    (:`NewEnumerator11`
      (`self.InitCamera`))
    (:`NewEnumerator12`
      (`self.SetUpScores`))
    (:`NewEnumerator4`
      (`self.InitGame`)
      (`self.BeginGame`))
    (:`NewEnumerator5`
      (set `self.CurrentState` "NewEnumerator5"))
    (:`NewEnumerator6`
      (`self.StorePlayerData`)
      (message `/Game/Student/Blueprint/Interfaces/BPI_GameData.DecrementGamesLeft` (`GameplayStatics.GetGameInstance`))
      (`self.OnNewState` "NewEnumerator8"))
    (:`NewEnumerator8`
      (`KismetSystemLibrary.Delay` 3.0)
      (`self.GoToScoreScreen`))))

(event `self.K2_PostLogin`
  (params (NewPlayer :type "PlayerController Object Reference"))
  ;[1 1 1] Login
  (`parent.K2_PostLogin` NewPlayer))

(event `self.K2_OnLogout`
  (params (ExitingController :type "Controller Object Reference"))
  ;[1 1 1] Login
  (`parent.K2_OnLogout` ExitingController))

(event `/Game/Student/Blueprint/Interfaces/BPI_ZombieSurvival.BeginEndGame`
  (`self.EndGame`))

(fn `EndGame`
  (bind _output_get (set `self.CurrentState` "NewEnumerator6"))
  (`self.OnNewState` _output_get)
  (bind _returnvalue (`|CreateWidget` "/Game/Student/Blueprint/Widgets/BPW_GameOver.BPW_GameOver_C"))
  (bind _output_get_2 (set `self.GameOver_0` _returnvalue))
  (`UserWidget.AddToViewport` _output_get_2 0))

(fn `GetPlayers`
  (returns (Players :type "Array of /Game/Student/Blueprint/Gameplay/Characters/BP_BaseTeamCharacter Object Reference"))
  (bind _players (`parent.GetPlayers`))
  (return _players))

(fn `Init`
  (set `self.CurrentState` "NewEnumerator0")
  (bind _data (message `/Game/Student/Blueprint/Interfaces/BPI_GameData.GetSetUpData` (`GameplayStatics.GetGameInstance`)))
  (bind _output_get (set `self.SetUpData` _data))
  (bind _outactors (`GameplayStatics.GetAllActorsOfClass` "/Game/Student/Blueprint/Gameplay/Camera/BP_MultiplayerCamera.BP_MultiplayerCamera_C"))
  (for _array_element _outactors
    (switch `/Game/Student/Blueprint/Data/E_GameModes` (`/Game/Student/Blueprint/Gameplay/Camera/BP_MultiplayerCamera.GameMode` _array_element)
      (:`NewEnumerator1`
        (set `self.Multiplayer Camera` _array_element)
        (break))))
  (`self.SetUpControllers` (break `/Game/Student/Blueprint/Data/S_SetUpData` _output_get))
  (`self.AssignPlayerOne`)
  (`self.OnNewState` "NewEnumerator3"))

(fn `InitCamera`
  (set `self.CurrentState` "NewEnumerator11")
  (`/Game/Student/Blueprint/Gameplay/Camera/BP_MultiplayerCamera.InitCamera` (`self.Multiplayer Camera`) (make `/Game/Student/Blueprint/Gameplay/Camera/S_CameraSettings` 600.0 3500.0 600.0 2.5 2.0) (`self.PlayerCharacters`))
  (`self.OnNewState` "NewEnumerator12"))

(fn `InitCharacters`
  (locals (currentCharacter :type "/Game/Student/Blueprint/Gameplay/Characters/BP_BaseTeamCharacter Object Reference") (currentController :type "/Game/Student/Blueprint/Controllers/PC_ArenaController Object Reference"))
  (set `self.CurrentState` "NewEnumerator2")
  (for (_array_element _array_index) (`self.PlayerControllers`)
    (set `local.currentController` _array_element)
    (bind _returnvalue (`|SpawnActorFromClass` "/Game/Student/Blueprint/Gameplay/Characters/BP_BaseTeamCharacter.BP_BaseTeamCharacter_C" (`KismetMathLibrary.MakeTransform` (`|GetArrayItem` (`self.SpawnPoints`) _array_index)) "AdjustIfPossibleButAlwaysSpawn" "OverrideRootScale" null null))
    (bind _output_get (set `local.currentCharacter` _returnvalue))
    (`KismetArrayLibrary.Array_Add` (`self.PlayerCharacters`) _output_get)
    (`Controller.Possess` (`local.currentController`) (`local.currentCharacter`))
    (`PlayerController.SetViewTargetWithBlend` (`local.currentController`) (`self.Multiplayer Camera`) 0.0 "VTBlend_Linear" 0.0 false)
    (`/Game/Student/Blueprint/Gameplay/Characters/BP_BaseTeamCharacter.GetComponentRefs` (`local.currentCharacter`))
    (set `/Game/Framework_Blueprints/Characters/BP_BaseCharacter.DefaultWeapons` (`self.DefaultWeapons`) (`local.currentCharacter`))
    (`/Game/Student/Blueprint/Interfaces/BPI_Init.InitActor` (`local.currentCharacter`))
    (`/Game/Student/Blueprint/Interfaces/BPI_TeamData.AssignTeam` (`local.currentCharacter`) "NewEnumerator2")
    (set `/Game/Student/Blueprint/Gameplay/Characters/BP_BaseTeamCharacter.DeathScorePenalty` 150 (`local.currentCharacter`)))
  (`self.OnBindToPlayerDeath`)
  (`self.OnBindToPlayerRespawn`)
  (`self.OnNewState` "NewEnumerator11"))

(fn `InitGame`
  (set `self.CurrentState` "NewEnumerator4")
  (bind _returnvalue (`GameplayStatics.GetActorOfClass` "/Game/Student/Blueprint/Gameplay/BossRush/Boss/BP_Boss.BP_Boss_C"))
  (bind _output_get (set `self.Boss` _returnvalue))
  (`/Game/Student/Blueprint/Interfaces/BPI_Init.InitActor` _output_get)
  (bind _outactors (`GameplayStatics.GetAllActorsOfClass` "/Game/Student/Blueprint/Gameplay/RandomWeaponSpawner.RandomWeaponSpawner_C"))
  (for _array_element _outactors
    (switch `/Game/Student/Blueprint/Data/E_GameModes` (`/Game/Student/Blueprint/Gameplay/RandomWeaponSpawner.GameMode` _array_element)
      (:`NewEnumerator2`
        (set `self.randomLootSpawner` _array_element)
        (break))))
  (`/Engine/EditorBlueprintResources/StandardMacros.IsValid` (`self.randomLootSpawner`)
    (:`Is Valid`
      (message `/Game/Student/Blueprint/Interfaces/BPI_Init.InitActor` (`self.randomLootSpawner`)))))

(fn `SetUpSpawnPoints`
  (locals (allPoints :type "Array of Vector Structure") (randIndies :type "Array of Integer"))
  (bind _setupdata_nplayers (break `/Game/Student/Blueprint/Data/S_SetUpData` (`self.SetUpData`)))
  (set `self.CurrentState` "NewEnumerator1")
  (bind _outactors (`GameplayStatics.GetAllActorsOfClass` "/Game/Student/Blueprint/Spawning/BP_PlayerSpawner.BP_PlayerSpawner_C"))
  (for _array_element _outactors
    (bind _gamemode (`/Game/Student/Blueprint/Spawning/BP_PlayerSpawner.GetGameModeSpawner` _array_element))
    (switch `/Game/Student/Blueprint/Data/E_GameModes` _gamemode
      (:`NewEnumerator1`
        (`KismetArrayLibrary.Array_Add` (`self.Playerspawns`) _array_element))))
  (bind _spawnpoints (`/Game/Student/Blueprint/Spawning/BP_PlayerSpawner.GetSpawnPoints` (`|GetArrayItem` (`self.Playerspawns`) (`KismetMathLibrary.RandomIntegerInRange` 0 (`KismetArrayLibrary.Array_LastIndex` (`self.Playerspawns`))))))
  (set `local.allPoints` _spawnpoints)
  (for _ (range 1 (+ _setupdata_nplayers 1))
    (`KismetArrayLibrary.Array_Add` (`local.randIndies`) (`KismetMathLibrary.RandomIntegerInRange` 0 (`KismetArrayLibrary.Array_LastIndex` _spawnpoints))))
  (for _array_element_2 (`local.randIndies`)
    (`KismetArrayLibrary.Array_Add` (`self.SpawnPoints`) (`|GetArrayItem` (`local.allPoints`) _array_element_2)))
  (`self.OnNewState` "NewEnumerator2"))

(fn `UserConstructionScript`)