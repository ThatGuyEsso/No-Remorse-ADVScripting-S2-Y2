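; King of the Hill game mode in which the team holding the capture zone scores on a repeating timer until time runs out.
; A chain of state-change events runs setup: random spawn points, characters split into player one versus the rest, shared camera, UI, capture zone and weapon spawner.
; Zone claimed and neutral events start and pause scoring, while separate timers refresh the countdown and trigger the game-over screen.
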(event `StartGameTimer`
  ;[1 1 1] Game timer management
  (set `self.CurrentState` "NewEnumerator5")
  (bind _returnvalue (`KismetSystemLibrary.K2_SetTimerDelegate` (delegate `OnUpdateTimer`) 0.2 true))
  (set `self.GameTimeHandle` _returnvalue)
  (bind _returnvalue_2 (`KismetSystemLibrary.K2_SetTimer` null "EndGame" (`self.GameTime`)))
  (set `self.ElapsedTimeHandle` _returnvalue_2))

(event `self.ReceiveBeginPlay`
  (add `self.OnNewState` (delegate `self.OnGameStateChange`))
  (`self.OnNewState` "NewEnumerator0"))

(event `OnUpdateTimer`
  (bind _returnvalue (`KismetMathLibrary.FCeil` (- (`self.GameTime`) (`KismetSystemLibrary.K2_GetTimerElapsedTimeHandle` (`self.ElapsedTimeHandle`)))))
  ;[1 1 1] Game timer management
  (switch `/Game/Student/Blueprint/Data/E_GameStates` (`self.CurrentState`)
    (:`NewEnumerator5`
      (`/Game/Student/Blueprint/Widgets/BPW_GameTimer.UpdateDisplay` (`self.GameTimer`) (`KismetMathLibrary.Clamp` _returnvalue 0 (`KismetMathLibrary.FTrunc` (`self.GameTime`))))
      (if (<= _returnvalue 0)
        (`KismetSystemLibrary.K2_PauseTimerHandle` (`self.GameTimeHandle`))))))

(event `self.OnGameStateChange`
  (params (newState :type "/Game/Student/Blueprint/Data/E_GameStates Enum" :default "NewEnumerator0"))
  (switch `/Game/Student/Blueprint/Data/E_GameStates` newState
    (:`NewEnumerator0`
      (`self.Init`))
    (:`NewEnumerator3`
      (`KismetSystemLibrary.PrintString` "Set up arena for King of the hill  gamemode ")
      (`self.OnNewState` "NewEnumerator1"))
    (:`NewEnumerator1`
      (`self.SetUpSpawnPoints`))
    (:`NewEnumerator2`
      (`self.InitCharacters`))
    (:`NewEnumerator11`
      (`self.InitCamera`))
    (:`NewEnumerator12`
      (`self.SetUpScores`))
    (:`NewEnumerator4`
      (`self.InitGame`)
      (`self.BeginGame`))
    (:`NewEnumerator5`
      (`self.StartGameTimer`))))

(event `self.K2_PostLogin`
  (params (NewPlayer :type "PlayerController Object Reference"))
  ;[1 1 1] Login
  (`parent.K2_PostLogin` NewPlayer))

(event `self.K2_OnLogout`
  (params (ExitingController :type "Controller Object Reference"))
  ;[1 1 1] Login
  (`parent.K2_OnLogout` ExitingController))

(event `BindToCaptureZone`
  ;[1 1 1] CApture zone point system
  (`/Engine/EditorBlueprintResources/StandardMacros.IsValid` (`self.captureZone`)
    (:`Is Valid`
      (add `/Game/Student/Blueprint/Gameplay/KTH/BP_CaptureZone.OnZoneClaimed` (`self.captureZone`) (delegate `BeginPlayer`))
      (add `/Game/Student/Blueprint/Gameplay/KTH/BP_CaptureZone.OnZoneNeutral` (`self.captureZone`) (delegate `StopScoreTimer`)))))

(event `StopScoreTimer`
  ;[1 1 1] CApture zone point system
  (`KismetSystemLibrary.K2_PauseTimerHandle` (`self.ScoreTimer`)))

(event `BeginPlayer`
  (params (ClaimingTeam :type "/Game/Student/Blueprint/Data/E_Teams Enum" :default "NewEnumerator0"))
  ;[1 1 1] CApture zone point system
  (set `self.TeamInControl` ClaimingTeam)
  (bind _returnvalue (`KismetSystemLibrary.K2_SetTimerDelegate` (delegate `BeginAddToTeamScore`) (`self.PointTime`) true))
  (set `self.ScoreTimer` _returnvalue))

(event `BeginAddToTeamScore`
  ;[1 1 1] CApture zone point system
  (`self.AddToTeamScore`))

(fn `AddToTeamScore`
  (for _array_element (`self.PlayerCharacters`)
    (bind _isonteam (`/Game/Student/Blueprint/Interfaces/BPI_TeamData.IsOnTeam` _array_element (`self.TeamInControl`)))
    (if _isonteam
      (message `/Game/Student/Blueprint/Gameplay/Characters/Interfaces/BPI_Scoreable.AddScore` _array_element (`self.controlPointScore`) null))))

(fn `AssignPlayersDifferentTeam`
  (for _array_element (`self.PlayerControllers`)
    (if (`/Game/Student/Blueprint/Controllers/PC_ArenaController.isPlayer1` _array_element)
      (bind _returnvalue (`Controller.K2_GetPawn` _array_element))
      (message `/Game/Student/Blueprint/Interfaces/BPI_TeamData.AssignTeam` _returnvalue "NewEnumerator0")
      (else
        (message `/Game/Student/Blueprint/Interfaces/BPI_TeamData.AssignTeam` _returnvalue "NewEnumerator1")))))

(fn `EndGame`
  (bind _output_get (set `self.CurrentState` "NewEnumerator6"))
  (`self.OnNewState` _output_get)
  (`/Game/Student/Blueprint/Widgets/BPW_GameTimer.UpdateDisplay` (`self.GameTimer`) 0)
  (bind _returnvalue (`|CreateWidget` "/Game/Student/Blueprint/Widgets/BPW_GameOver.BPW_GameOver_C"))
  (bind _output_get_2 (set `self.GameOver` _returnvalue))
  (`UserWidget.AddToViewport` _output_get_2 0))

(fn `GetGameType`
  (returns (GameModeType :type "/Game/Student/Blueprint/Data/E_GameModes Enum"))
  (return "NewEnumerator2"))

(fn `Init`
  (set `self.CurrentState` "NewEnumerator0")
  (bind _data (message `/Game/Student/Blueprint/Interfaces/BPI_GameData.GetSetUpData` (`GameplayStatics.GetGameInstance`)))
  (bind _output_get (set `self.SetUpData` _data))
  (bind _outactors (`GameplayStatics.GetAllActorsOfClass` "/Game/Student/Blueprint/Gameplay/Camera/BP_MultiplayerCamera.BP_MultiplayerCamera_C"))
  (for _array_element _outactors
    (switch `/Game/Student/Blueprint/Data/E_GameModes` (`/Game/Student/Blueprint/Gameplay/Camera/BP_MultiplayerCamera.GameMode` _array_element)
      (:`NewEnumerator2`
        (set `self.Multiplayer Camera` _array_element)
        (break))))
  (`self.SetUpControllers` (break `/Game/Student/Blueprint/Data/S_SetUpData` _output_get))
  (`self.AssignPlayerOne`)
  (`self.OnNewState` "NewEnumerator3"))

(fn `InitCamera`
  (set `self.CurrentState` "NewEnumerator11")
  (`/Game/Student/Blueprint/Gameplay/Camera/BP_MultiplayerCamera.InitCamera` (`self.Multiplayer Camera`) (make `/Game/Student/Blueprint/Gameplay/Camera/S_CameraSettings` 500.0 3500.0 1000.0 2.5 2.0) (`self.PlayerCharacters`))
  (`self.OnNewState` "NewEnumerator12"))

(fn `InitCharacters`
  (locals (currentCharacter :type "/Game/Student/Blueprint/Gameplay/Characters/BP_BaseTeamCharacter Object Reference") (currentController :type "/Game/Student/Blueprint/Controllers/PC_ArenaController Object Reference"))
  (set `self.CurrentState` "NewEnumerator2")
  (for (_array_element _array_index) (`self.PlayerControllers`)
    (set `local.currentController` _array_element)
    (bind _returnvalue (`|SpawnActorFromClass` "/Game/Student/Blueprint/Gameplay/Characters/BP_BaseTeamCharacter.BP_BaseTeamCharacter_C" (`KismetMathLibrary.MakeTransform` (`|GetArrayItem` (`self.SpawnPoints`) _array_index)) "Undefined" "OverrideRootScale" null null))
    (set `local.currentCharacter` _returnvalue)
    (`KismetArrayLibrary.Array_Add` (`self.PlayerCharacters`) _returnvalue)
    (`Controller.Possess` (`local.currentController`) _returnvalue)
    (`PlayerController.SetViewTargetWithBlend` (`local.currentController`) (`self.Multiplayer Camera`) 0.0 "VTBlend_Linear" 0.0 false)
    (`/Game/Student/Blueprint/Gameplay/Characters/BP_BaseTeamCharacter.GetComponentRefs` _returnvalue)
    (set `/Game/Framework_Blueprints/Characters/BP_BaseCharacter.DefaultWeapons` (`self.DefaultWeapons`) (`local.currentCharacter`))
    (`/Game/Student/Blueprint/Interfaces/BPI_Init.InitActor` (`local.currentCharacter`)))
  (`self.OnBindToPlayerDeath`)
  (`self.OnBindToPlayerRespawn`)
  (`self.AssignPlayersDifferentTeam`)
  (`self.OnNewState` "NewEnumerator11"))

(fn `InitGame`
  (set `self.CurrentState` "NewEnumerator4")
  (bind _returnvalue (`|CreateWidget` "/Game/Student/Blueprint/Widgets/BPW_GameTimer.BPW_GameTimer_C"))
  (bind _output_get (set `self.GameTimer` _returnvalue))
  (`UserWidget.AddToViewport` _output_get 0)
  (bind _returnvalue_2 (`GameplayStatics.GetActorOfClass` "/Game/Student/Blueprint/Gameplay/KTH/BP_CaptureZone.BP_CaptureZone_C"))
  (bind _output_get_2 (set `self.captureZone` _returnvalue_2))
  (`/Engine/EditorBlueprintResources/StandardMacros.IsValid` _output_get_2
    (:`Is Valid`
      (`/Game/Student/Blueprint/Interfaces/BPI_Init.InitActor` _output_get_2)
      (`self.BindToCaptureZone`)
      (bind _outactors (`GameplayStatics.GetAllActorsOfClass` "/Game/Student/Blueprint/Gameplay/KTH/RandomWeaponSpawner.RandomWeaponSpawner_C"))
      (for _array_element _outactors
        (switch `/Game/Student/Blueprint/Data/E_GameModes` (`/Game/Student/Blueprint/Gameplay/KTH/RandomWeaponSpawner.GameMode` _array_element)
          (:`NewEnumerator2`
            (set `self.randomLootSpawner` _array_element)
            (break))))
      (`/Engine/EditorBlueprintResources/StandardMacros.IsValid` (`self.randomLootSpawner`)
        (:`Is Valid`
          (message `/Game/Student/Blueprint/Interfaces/BPI_Init.InitActor` (`self.randomLootSpawner`)))))))

(fn `SetUpSpawnPoints`
  (locals (randIndies :type "Array of Integer") (allPoints :type "Array of Vector Structure"))
  (bind _setupdata_nplayers (break `/Game/Student/Blueprint/Data/S_SetUpData` (`self.SetUpData`)))
  (set `self.CurrentState` "NewEnumerator1")
  (bind _outactors (`GameplayStatics.GetAllActorsOfClass` "/Game/Student/Blueprint/Spawning/BP_PlayerSpawner.BP_PlayerSpawner_C"))
  (for _array_element _outactors
    (bind _gamemode (`/Game/Student/Blueprint/Spawning/BP_PlayerSpawner.GetGameModeSpawner` _array_element))
    (switch `/Game/Student/Blueprint/Data/E_GameModes` _gamemode
      (:`NewEnumerator2`
        (`KismetArrayLibrary.Array_Add` (`self.Playerspawns`) _array_element))))
  (bind _spawnpoints (`/Game/Student/Blueprint/Spawning/BP_PlayerSpawner.GetSpawnPoints` (`|GetArrayItem` (`self.Playerspawns`) (`KismetMathLibrary.RandomIntegerInRange` 0 (`KismetArrayLibrary.Array_LastIndex` (`self.Playerspawns`))))))
  (set `local.allPoints` _spawnpoints)
  (for _ (range 1 (+ _setupdata_nplayers 1))
    (`KismetArrayLibrary.Array_Add` (`local.randIndies`) (`KismetMathLibrary.RandomIntegerInRange` 0 (`KismetArrayLibrary.Array_LastIndex` _spawnpoints))))
  (for _array_element_2 (`local.randIndies`)
    (`KismetArrayLibrary.Array_Add` (`self.SpawnPoints`) (`|GetArrayItem` (`local.allPoints`) _array_element_2)))
  (`self.OnNewState` "NewEnumerator2"))

(fn `UserConstructionScript`)