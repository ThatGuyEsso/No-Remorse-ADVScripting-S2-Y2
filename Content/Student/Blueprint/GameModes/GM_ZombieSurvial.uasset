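; Game mode for local-multiplayer Zombie Survival, running the arena from player creation to score screen.
; An event-dispatched state chain sets up spawns, characters, shared camera and UI, then spawns BP_WaveManager with the zombie spawners and runs a start countdown.
; It respawns dead players at random spawners, updates the camera's alive count and broadcasts zombie-capacity changes.
; Ending shows game over, stores scores in the GameInstance and opens ScoreScreen.
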(event `self.ReceiveBeginPlay`
  (add `self.OnNewState` (delegate `OnGameStateChange`))
  (`self.OnNewState` "NewEnumerator0"))

(event `OnGameStateChange` :!signature `self.OnNewState`
  (params (newState :type "/Game/Student/Blueprint/Data/E_GameStates Enum" :default "NewEnumerator0"))
  ;[1 1 1] Initiation Chain
  (switch `/Game/Student/Blueprint/Data/E_GameStates` newState
    (:`NewEnumerator0`
      (`self.Init`))
    (:`NewEnumerator3`
      (`KismetSystemLibrary.PrintString` "Set up arena for zombie gamemode ")
      (`self.OnNewState` "NewEnumerator1"))
    (:`NewEnumerator1`
      (`self.SetUpSpawnPoints`))
    (:`NewEnumerator2`
      (`self.InitCharacters`))
    (:`NewEnumerator11`
      (`self.InitCamera`))
    (:`NewEnumerator12`
      (`self.SetUpScores`))
    (:`NewEnumerator4`
      (`self.InitGame`)
      (`self.BeginGame`))
    (:`NewEnumerator5`
      (set `self.CurrentState` "NewEnumerator5"))
    (:`NewEnumerator6`
      (`self.StorePlayerData`)
      (message `/Game/Student/Blueprint/Interfaces/BPI_GameData.DecrementGamesLeft` (`GameplayStatics.GetGameInstance`))
      (`self.OnNewState` "NewEnumerator8"))
    (:`NewEnumerator8`
      (`KismetSystemLibrary.Delay` 3.0)
      (`self.GoToScoreScreen`))))

(event `BeginGame`
  (bind _returnvalue (`|CreateWidget` "/Game/Student/Blueprint/Widgets/BPW_GameStartCountDOwn.BPW_GameStartCountDown_C"))
  (bind _output_get (set `self.countDownUIRef` _returnvalue))
  (`UserWidget.AddToViewport` _output_get 0)
  (bind _returnvalue_2 (`KismetSystemLibrary.K2_SetTimerDelegate` (delegate `StartGame`) (`self.GameCountDownTime`)))
  (set `self.CountDownHandle` _returnvalue_2)
  (bind _returnvalue_3 (`KismetSystemLibrary.K2_SetTimerDelegate` (delegate `GameStartCountDown`) 0.2 true))
  (set `self.DisplayUpdateTimer` _returnvalue_3))

(event `GameStartCountDown`
  (`/Game/Student/Blueprint/Widgets/BPW_GameStartCountDOwn.UpdateTimer` (`self.countDownUIRef`) (`KismetMathLibrary.FCeil` (- (`self.GameCountDownTime`) (`KismetSystemLibrary.K2_GetTimerElapsedTimeHandle` (`self.CountDownHandle`))))))

(event `StartGame`
  (`self.OnNewState` "NewEnumerator5")
  (`Widget.RemoveFromParent` (`self.countDownUIRef`))
  (`KismetSystemLibrary.K2_PauseTimerHandle` (`self.DisplayUpdateTimer`)))

(event `OnBindToPlayerDeath`
  (for _array_element (`self.PlayerCharacters`)
    (add `/Game/Student/Blueprint/Gameplay/Characters/BP_BaseTeamCharacter.OnPlayerDied` _array_element (delegate `OnPlayerDied`))))

(event `self.K2_PostLogin`
  (params (NewPlayer :type "PlayerController Object Reference"))
  ;[1 1 1] Controller Log in
  (bind _aspc_arena_controller (cast `/Game/Student/Blueprint/Controllers/PC_ArenaController` NewPlayer))
  (set `PlayerController.bShowMouseCursor` false _aspc_arena_controller)
  (`KismetArrayLibrary.Array_Add` (`self.PlayerControllers`) _aspc_arena_controller))

(event `self.K2_OnLogout`
  (params (ExitingController :type "Controller Object Reference"))
  ;[1 1 1] Controller Log in
  (bind _aspc_arena_controller (cast `/Game/Student/Blueprint/Controllers/PC_ArenaController` ExitingController))
  (`KismetArrayLibrary.Array_RemoveItem` (`self.PlayerControllers`) _aspc_arena_controller))

(event `OnPlayerDied`
  (params (Player :type "Actor Object Reference"))
  (bind _nplayersalive (`self.GetNPlayersAlive`))
  (`/Game/Student/Blueprint/Gameplay/Camera/BP_MultiplayerCamera.UpdateAlivePlayers` (`self.Multiplayer Camera`) _nplayersalive)
  (`/Game/Student/Blueprint/Spawning/BP_PlayerSpawner.RespawnPlayer` (`|GetArrayItem` (`self.Playerspawns`) (`KismetMathLibrary.RandomInteger` (`KismetArrayLibrary.Array_LastIndex` (`self.Playerspawns`)))) Player))

(event `OnBindToPlayerRespawn`
  (for _array_element (`self.PlayerCharacters`)
    (add `/Game/Student/Blueprint/Gameplay/Characters/BP_BaseTeamCharacter.OnPlayerSpawned` _array_element (delegate `OnPlayerRespawned`))))

(event `OnPlayerRespawned`
  (params (character :type "Actor Object Reference"))
  (bind _nplayersalive (`self.GetNPlayersAlive`))
  (`/Game/Student/Blueprint/Gameplay/Camera/BP_MultiplayerCamera.UpdateAlivePlayers` (`self.Multiplayer Camera`) _nplayersalive))

(event `/Game/Student/Blueprint/Interfaces/BPI_ZombieSurvival.ZombieKilled`
  ;[1 1 1] Zombie Updates events (When they are added or removed)
  (bind _result (`/Engine/EditorBlueprintResources/StandardMacros.DecrementInt` (`self.ZombieCount`))
    (:`  `
      (if (< _result (`self.MaxZombiesCount`))
        (`self.OnNotAtEnemyCapacity`)))))

(event `/Game/Student/Blueprint/Interfaces/BPI_ZombieSurvival.NewZombieSpawned`
  ;[1 1 1] Zombie Updates events (When they are added or removed)
  (bind _result (`/Engine/EditorBlueprintResources/StandardMacros.IncrementInt` (`self.ZombieCount`))
    (:`  `
      (if (>= _result (`self.MaxZombiesCount`))
        (`self.OnEnemyCapacityReached`)))))

(event `/Game/Student/Blueprint/Interfaces/BPI_ZombieSurvival.RefreshZombieLimit`
  ;[1 1 1] Zombie Updates events (When they are added or removed)
  (if (< (`self.ZombieCount`) (`self.MaxZombiesCount`))
    (`self.OnNotAtEnemyCapacity`)
    (else
      (`self.OnEnemyCapacityReached`))))

(event `/Game/Student/Blueprint/Interfaces/BPI_ZombieSurvival.SetMaxZombies`
  (params (NewMaxZombies :type Integer))
  ;[1 1 1] Increment Zombies
  (set `self.MaxZombiesCount` NewMaxZombies))

(event `/Game/Student/Blueprint/Interfaces/BPI_ZombieSurvival.BeginEndGame`
  (`self.EndGame`))

(fn `AssignPlayerOne`
  (locals (NewLocalVar_0 :type Integer))
  (bind _setupdata (`self.SetUpData`))
  (set `local.NewLocalVar_0` (break `/Game/Student/Blueprint/Data/S_ControllerMap` (`.PlayerOne_14_E6533503497D0A7DBE94BC84CA1C63B2` (break `/Game/Student/Blueprint/Data/S_SetUpData` _setupdata))))
  (for _array_element (`self.PlayerControllers`)
    (if (== (`GameplayStatics.GetPlayerControllerID` _array_element) (break `/Game/Student/Blueprint/Data/S_ControllerMap` (`.PlayerOne_14_E6533503497D0A7DBE94BC84CA1C63B2` (break `/Game/Student/Blueprint/Data/S_SetUpData` _setupdata))))
      (set `/Game/Student/Blueprint/Controllers/PC_ArenaController.isPlayer1` true _array_element)
      (else
        (set `/Game/Student/Blueprint/Controllers/PC_ArenaController.isPlayer1` false _array_element)))))

(fn `EndGame`
  (bind _output_get (set `self.CurrentState` "NewEnumerator6"))
  (`self.OnNewState` _output_get)
  (bind _returnvalue (`|CreateWidget` "/Game/Student/Blueprint/Widgets/BPW_GameOver.BPW_GameOver_C"))
  (bind _output_get_2 (set `self.GameOver` _returnvalue))
  (`UserWidget.AddToViewport` _output_get_2 0))

(fn `GetGameModeRef`
  (returns (ZombieGameMode :type "/Game/Student/Blueprint/GameModes/GM_ZombieSurvial Object Reference"))
  (return self))

(fn `GetGamesTotal`
  (returns (totalGames :type Integer))
  (return 0))

(fn `GetGameType`
  (returns (GameModeType :type "/Game/Student/Blueprint/Data/E_GameModes Enum"))
  (return "NewEnumerator0"))

(fn `GetKTHGameModeRef`
  (returns (KTH :type "/Game/Student/Blueprint/GameModes/GM_KingOfTheHill Object Reference"))
  (return null))

(fn `GetNextGameMode`
  (params (index :type Integer))
  (returns (GameMode :type "/Game/Student/Blueprint/Data/E_GameModes Enum"))
  (return "NewEnumerator0"))

(fn `GetNPlayersAlive`
  (returns (nPlayersAlive :type Integer))
  (locals (nAlive :type Integer))
  (for _array_element (`self.PlayerCharacters`)
    (bind _isalive (`/Game/Student/Blueprint/Gameplay/Characters/BP_BaseTeamCharacter.GetIsAlive` _array_element))
    (if _isalive
      (`/Engine/EditorBlueprintResources/StandardMacros.IncrementInt` (`local.nAlive`))))
  (return (`local.nAlive`)))

(fn `GetNumberOfGamesLeft`
  (returns (GamesLeft :type Integer))
  (return 0))

(fn `GetPlayerData`
  (returns (PlayerOne :type "/Game/Student/Blueprint/Data/S_PlayerData Structure") (PlayerTwo :type "/Game/Student/Blueprint/Data/S_PlayerData Structure"))
  (return))

(fn `GetPlayerOne`
  (returns (PlayerOneController :type "/Game/Student/Blueprint/Controllers/PC_ArenaController Object Reference"))
  (for _array_element (`self.PlayerControllers`)
    (if (`/Game/Student/Blueprint/Controllers/PC_ArenaController.isPlayer1` _array_element)
      (return _array_element))))

(fn `GetPlayers`
  (returns (Players :type "Array of /Game/Student/Blueprint/Gameplay/Characters/BP_BaseTeamCharacter Object Reference"))
  (return (`self.PlayerCharacters`)))

(fn `GetPlayersAlive`
  (returns (players :type "Array of /Game/Student/Blueprint/Gameplay/Characters/BP_BaseTeamCharacter Object Reference"))
  (locals (alivePLayers :type "Array of /Game/Student/Blueprint/Gameplay/Characters/BP_BaseTeamCharacter Object Reference"))
  (for _array_element (`self.PlayerCharacters`)
    (bind _isalive (`/Game/Student/Blueprint/Gameplay/Characters/BP_BaseTeamCharacter.GetIsAlive` _array_element))
    (if _isalive
      (`KismetArrayLibrary.Array_Add` (`local.alivePLayers`) _array_element)))
  (return (`local.alivePLayers`)))

(fn `GetSetUpData`
  (returns (Data :type "/Game/Student/Blueprint/Data/S_SetUpData Structure"))
  (return))

(fn `GetTeam`
  (returns (Team :type "/Game/Student/Blueprint/Data/E_Teams Enum"))
  (return "NewEnumerator0"))

(fn `GoToScoreScreen`
  (for _array_element (`self.PlayerControllers`)
    (`GameplayStatics.RemovePlayer` _array_element true))
  (`GameplayStatics.OpenLevel` "ScoreScreen"))

(fn `Init`
  (set `self.CurrentState` "NewEnumerator0")
  (bind _data (message `/Game/Student/Blueprint/Interfaces/BPI_GameData.GetSetUpData` (`GameplayStatics.GetGameInstance`)))
  (bind _output_get (set `self.SetUpData` _data))
  (bind _outactors (`GameplayStatics.GetAllActorsOfClass` "/Game/Student/Blueprint/Gameplay/Camera/BP_MultiplayerCamera.BP_MultiplayerCamera_C"))
  (for _array_element _outactors
    (switch `/Game/Student/Blueprint/Data/E_GameModes` (`/Game/Student/Blueprint/Gameplay/Camera/BP_MultiplayerCamera.GameMode` _array_element)
      (:`NewEnumerator0`
        (set `self.Multiplayer Camera` _array_element)
        (break))))
  (`self.SetUpControllers` (break `/Game/Student/Blueprint/Data/S_SetUpData` _output_get))
  (`self.AssignPlayerOne`)
  (`self.OnNewState` "NewEnumerator3"))

(fn `InitCamera`
  (set `self.CurrentState` "NewEnumerator11")
  (`/Game/Student/Blueprint/Gameplay/Camera/BP_MultiplayerCamera.InitCamera` (`self.Multiplayer Camera`) (make `/Game/Student/Blueprint/Gameplay/Camera/S_CameraSettings` 750.0 3500.0 750.0 2.5 2.0 3) (`self.PlayerCharacters`))
  (`self.OnNewState` "NewEnumerator12"))

(fn `InitCharacters`
  (locals (currentController :type "/Game/Student/Blueprint/Controllers/PC_ArenaController Object Reference") (currentCharacter :type "/Game/Student/Blueprint/Gameplay/Characters/BP_BaseTeamCharacter Object Reference"))
  (set `self.CurrentState` "NewEnumerator2")
  (for (_array_element _array_index) (`self.PlayerControllers`)
    (set `local.currentController` _array_element)
    (bind _returnvalue (`|SpawnActorFromClass` "/Game/Student/Blueprint/Gameplay/Characters/BP_BaseTeamCharacter.BP_BaseTeamCharacter_C" (`KismetMathLibrary.MakeTransform` (`|GetArrayItem` (`self.SpawnPoints`) _array_index)) "Undefined" "OverrideRootScale" null null))
    (set `local.currentCharacter` _returnvalue)
    (`KismetArrayLibrary.Array_Add` (`self.PlayerCharacters`) _returnvalue)
    (`Controller.Possess` (`local.currentController`) _returnvalue)
    (`PlayerController.SetViewTargetWithBlend` (`local.currentController`) (`self.Multiplayer Camera`) 0.0 "VTBlend_Linear" 0.0 false)
    (`/Game/Student/Blueprint/Gameplay/Characters/BP_BaseTeamCharacter.GetComponentRefs` _returnvalue)
    (set `/Game/Framework_Blueprints/Characters/BP_BaseCharacter.DefaultWeapons` (`self.DefaultWeapons`) (`local.currentCharacter`))
    (`/Game/Student/Blueprint/Interfaces/BPI_Init.InitActor` (`local.currentCharacter`))
    (`/Game/Student/Blueprint/Interfaces/BPI_TeamData.AssignTeam` (`local.currentCharacter`) "NewEnumerator2"))
  (`self.OnBindToPlayerDeath`)
  (`self.OnBindToPlayerRespawn`)
  (`self.OnNewState` "NewEnumerator11"))

(fn `InitGame`
  (locals (spawners :type "Array of /Game/Student/Blueprint/Gameplay/ZombieSurvival/BP_ZombieSpawner Object Reference"))
  (set `self.CurrentState` "NewEnumerator4")
  (bind _outactors (`GameplayStatics.GetAllActorsOfClass` "/Game/Student/Blueprint/Gameplay/ZombieSurvival/BP_ZombieSpawner.BP_ZombieSpawner_C"))
  (set `local.spawners` _outactors)
  (bind _returnvalue (`|SpawnActorFromClass` "/Game/Student/Blueprint/Spawning/BP_WaveManager.BP_WaveManager_C" (`KismetMathLibrary.MakeTransform` (0.0 0.0 0.0)) "Undefined" "OverrideRootScale" null null))
  (message `/Game/Student/Blueprint/Interfaces/BPI_Init.InitActor` _returnvalue)
  (set `/Game/Student/Blueprint/Spawning/BP_WaveManager.spawners` (`local.spawners`) _returnvalue))

(fn `IsAtZombieCapacity`
  (returns (IsAtCapacity :type Boolean))
  (return false))

(fn `IsGameRunning`
  (returns (isRunnning :type Boolean))
  (return (`|EnumEquality` (`self.CurrentState`) "NewEnumerator5")))

(fn `IsOnTeam`
  (params (CallerTeam :type "/Game/Student/Blueprint/Data/E_Teams Enum" :default "NewEnumerator0"))
  (returns (IsOnTeam :type Boolean))
  (return false))

(fn `SetUpControllers`
  (params (nPlayers :type Integer))
  (`GameplayStatics.RemovePlayer` (`GameplayStatics.GetPlayerController` 0) true)
  (for _ (range nPlayers)
    (`GameplayStatics.CreatePlayer` -1)))

(fn `SetUpScores`
  (set `self.CurrentState` "NewEnumerator12")
  (bind _returnvalue (`|CreateWidget` "/Game/Student/Blueprint/Widgets/BPW_PlayerDIsplay.BPW_PlayerDIsplay_C"))
  (`UserWidget.AddToViewport` _returnvalue 0)
  (for _array_element (`self.PlayerControllers`)
    (`/Game/Student/Blueprint/Controllers/PC_ArenaController.SetPlayerDisplay` _array_element _returnvalue))
  (`self.OnNewState` "NewEnumerator4"))

(fn `SetUpSpawnPoints`
  (set `self.CurrentState` "NewEnumerator1")
  (bind _outactors (`GameplayStatics.GetAllActorsOfClass` "/Game/Student/Blueprint/Spawning/BP_PlayerSpawner.BP_PlayerSpawner_C"))
  (for _array_element _outactors
    (bind _gamemode (`/Game/Student/Blueprint/Spawning/BP_PlayerSpawner.GetGameModeSpawner` _array_element))
    (switch `/Game/Student/Blueprint/Data/E_GameModes` _gamemode
      (:`NewEnumerator0`
        (`KismetArrayLibrary.Array_Add` (`self.Playerspawns`) _array_element))))
  (for _array_element_2 (`self.Playerspawns`)
    (bind _gamemode_2 (`/Game/Student/Blueprint/Spawning/BP_PlayerSpawner.GetGameModeSpawner` _array_element_2))
    (switch `/Game/Student/Blueprint/Data/E_GameModes` _gamemode_2
      (:`NewEnumerator0`
        (bind _spawnpoints (`/Game/Student/Blueprint/Spawning/BP_PlayerSpawner.GetSpawnPoints` _array_element_2))
        (for _index (range 2)
          (`KismetArrayLibrary.Array_Add` (`self.SpawnPoints`) (`|GetArrayItem` _spawnpoints _index)))
        (break))))
  (`self.OnNewState` "NewEnumerator2"))

(fn `StorePlayerData`
  (bind _returnvalue (`GameplayStatics.GetGameInstance`))
  (for _array_element (`self.PlayerControllers`)
    (bind _playerscore (message `/Game/Student/Blueprint/Gameplay/Characters/Interfaces/BPI_Scoreable.GetScore` (`Controller.K2_GetPawn` _array_element)))
    (if (`/Game/Student/Blueprint/Controllers/PC_ArenaController.isPlayer1` _array_element)
      (message `/Game/Student/Blueprint/Interfaces/BPI_GameData.UpdatePlayerOneData` _returnvalue (make `/Game/Student/Blueprint/Data/S_PlayerData` _playerscore (`KismetMathLibrary.Conv_LinearColorToColor` (`KismetMathLibrary.LinearColor_ToNewOpacity` (struct :`R` 0.449831 :`G` 0.00973 :`B` 0.504167 :`A` 1.0) 1.0)) true))
      (else
        (message `/Game/Student/Blueprint/Interfaces/BPI_GameData.UpdatePlayerTwoData` _returnvalue (make `/Game/Student/Blueprint/Data/S_PlayerData` _playerscore (`KismetMathLibrary.Conv_LinearColorToColor` (`KismetMathLibrary.LinearColor_ToNewOpacity` (struct :`R` 0.087498 :`G` 1.0 :`A` 1.0) 1.0))))))))

(fn `UserConstructionScript`)