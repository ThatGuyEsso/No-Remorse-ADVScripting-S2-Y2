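; BP_TeamPistol is a pistol weapon that characters fire and that can also exist as a falling pickup.
; Fire spawns a BP_TeamProjectile at the character's fire point, passing its team, armour colour and fixed damage.
; While dropping, Tick lowers it until its DropCollider overlaps something; a successful player Pickup then destroys the actor.
; BeginPlay removes that collider on non-dropped pistols, and Init refills ammo to the starting amount.
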(event `self.ReceiveBeginPlay`
  (`parent.ReceiveBeginPlay`)
  (if (not (`self.isDropping`))
    (`ActorComponent.K2_DestroyComponent` (`self.DropCollider`))))

(event `self.DropCollider.OnComponentBeginOverlap`
  (params (OverlappedComponent :type "PrimitiveComponent Object Reference") (OtherActor :type "Actor Object Reference") (OtherComp :type "PrimitiveComponent Object Reference") (OtherBodyIndex :type Integer) (bFromSweep :type Boolean) (SweepResult :type "HitResult Structure (by ref)"))
  (set `self.isDropping` false)
  (if (`self.ActorHasTag` OtherActor "Player")
    (bind _success (`self.Pickup` OtherActor))
    (if _success
      (`self.K2_DestroyActor`))))

(event `self.ReceiveTick`
  (params (DeltaSeconds :type "Float (single-precision)"))
  (bind (_returnvalue_x _returnvalue_y _returnvalue_z) (`KismetMathLibrary.BreakVector` (`self.K2_GetActorLocation`)))
  (if (`self.isDropping`)
    (`self.K2_SetActorLocation` (`KismetMathLibrary.MakeVector` _returnvalue_x _returnvalue_y (- _returnvalue_z (* DeltaSeconds (`self.dropSpeed`)))))))

(fn `Fire`
  (bind _character (`self.Character`))
  (bind (_newparam_location _newparam_rotation) (`KismetMathLibrary.BreakTransform` (`/Game/Framework_Blueprints/Characters/BP_BaseCharacter.GetFirePoint` (`self.Character`))))
  (bind _team (message `/Game/Student/Blueprint/Interfaces/BPI_TeamData.GetTeam` _character))
  (`|SpawnActorFromClass` "/Game/Student/Blueprint/Gameplay/Weapons/BP_TeamProjectile.BP_TeamProjectile_C" (`KismetMathLibrary.MakeTransform` _newparam_location _newparam_rotation) "AlwaysSpawn" "OverrideRootScale" _character _team (`/Game/Framework_Blueprints/Characters/BP_BaseCharacter.ArmourColour` _character) 20.0 _character))

(fn `Init`
  (params (Character :type "/Game/Framework_Blueprints/Characters/BP_BaseCharacter Object Reference"))
  (`parent.Init` Character)
  (set `self.Ammo` (`self.startingAmmo`)))

(fn `UserConstructionScript`
  (`parent.UserConstructionScript`))