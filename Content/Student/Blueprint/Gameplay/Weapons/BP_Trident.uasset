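; BP_Trident is a weapon Blueprint that fires a spread of team projectiles from three fire points.
; Init calls the parent, sets the Trident starting ammo and registers the three fire point components.
; Fire spawns a scaled-down BP_TeamProjectile at each point along its forward vector, so component orientation sets the pattern.
; Each projectile receives the owning character's team and armour colour, plus the weapon's damage.
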(fn `Fire`
  (bind _character (`self.Character`))
  ;[1 1 1] Depending on the number of projectiles add yaw rotation for each bullet to create a spray effect.
  (for _array_element (`self.firePoints`)
    (bind _team (message `/Game/Student/Blueprint/Interfaces/BPI_TeamData.GetTeam` _character))
    (`|SpawnActorFromClass` "/Game/Student/Blueprint/Gameplay/Weapons/BP_TeamProjectile.BP_TeamProjectile_C" (`KismetMathLibrary.MakeTransform` (`SceneComponent.K2_GetComponentLocation` _array_element) (`KismetMathLibrary.MakeRotFromX` (`SceneComponent.GetForwardVector` _array_element)) (0.75 0.75 0.75)) "AlwaysSpawn" "OverrideRootScale" _character _team (`/Game/Framework_Blueprints/Characters/BP_BaseCharacter.ArmourColour` _character) (`self.Damage`) _character))
  (return))

(fn `Init`
  (params (Character :type "/Game/Framework_Blueprints/Characters/BP_BaseCharacter Object Reference"))
  (`parent.Init` Character)
  (set `self.Ammo` (`self.TridentStartingAmmo`))
  (`KismetArrayLibrary.Array_Add` (`self.firePoints`) (`self.MainFP`))
  (`KismetArrayLibrary.Array_Add` (`self.firePoints`) (`self.FP`))
  (`KismetArrayLibrary.Array_Add` (`self.firePoints`) (`self.Fp2`)))

(fn `UserConstructionScript`
  (`parent.UserConstructionScript`))