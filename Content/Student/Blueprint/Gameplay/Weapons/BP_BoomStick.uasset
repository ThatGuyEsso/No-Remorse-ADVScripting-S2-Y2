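; BP_BoomStick is a shotgun-style weapon that fires a horizontal spray of team projectiles.
; Fire spawns one BP_TeamProjectile per AmmoPerShot at the character's fire point, stepping each one's yaw by an even fraction of Spread to form a fan.
; Each projectile receives the character's team, armour colour and instigator, plus the weapon's damage.
; Init runs the parent setup, then sets Ammo to the BoomStick's starting amount.
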(fn `Fire`
  (bind _ammopershot (`self.AmmoPerShot`))
  (bind _character (`self.Character`))
  (bind _newparam_location (`KismetMathLibrary.BreakTransform` (`/Game/Framework_Blueprints/Characters/BP_BaseCharacter.GetFirePoint` (`self.Character`))))
  (bind _returnvalue (/ (`self.spread`) (`self.AmmoPerShot`)))
  (bind (_newparam_location_2 _newparam_rotation) (`KismetMathLibrary.BreakTransform` (`/Game/Framework_Blueprints/Characters/BP_BaseCharacter.GetFirePoint` (`self.Character`))))
  ;[1 1 1] Depending on the number of projectiles add yaw rotation for each bullet to create a spray effect.
  (for _index (range 1 (+ _ammopershot 1))
    (bind _team (message `/Game/Student/Blueprint/Interfaces/BPI_TeamData.GetTeam` _character))
    (`|SpawnActorFromClass` "/Game/Student/Blueprint/Gameplay/Weapons/BP_TeamProjectile.BP_TeamProjectile_C" (`KismetMathLibrary.MakeTransform` _newparam_location (`KismetMathLibrary.ComposeRotators` _newparam_rotation (`KismetMathLibrary.MakeRotator` 0.0 0.0 (+ (- 0.0 (* (/ _ammopershot 2) (`KismetMathLibrary.Conv_IntToDouble` _returnvalue))) (* _returnvalue (`KismetMathLibrary.Conv_IntToDouble` _index)))))) "AlwaysSpawn" "OverrideRootScale" _character _team (`/Game/Framework_Blueprints/Characters/BP_BaseCharacter.ArmourColour` _character) (`self.Damage`) _character))
  (return))

(fn `Init`
  (params (Character :type "/Game/Framework_Blueprints/Characters/BP_BaseCharacter Object Reference"))
  (`parent.Init` Character)
  (set `self.Ammo` (`self.BoomStickStartingAmmo`)))

(fn `UserConstructionScript`
  (`parent.UserConstructionScript`))