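; Camera zone trigger: a sphere that tracks whether all living players, identified by the "Player" tag, are inside it.
; Overlaps adjust a clamped count, calling enter dispatchers when it equals the alive count and exit dispatchers on departures leaving it different.
; Init assumes everyone starts inside and scales the radius by a multiplier.
; Separate functions update the alive count and add players found by a sphere trace.
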(event `self.Sphere.OnComponentBeginOverlap`
  (params (OverlappedComponent :type "PrimitiveComponent Object Reference") (OtherActor :type "Actor Object Reference") (OtherComp :type "PrimitiveComponent Object Reference") (OtherBodyIndex :type Integer) (bFromSweep :type Boolean) (SweepResult :type "HitResult Structure (by ref)"))
  (if (`self.ActorHasTag` OtherActor "Player")
    (`self.IncrementPlayers`)
    (if (== (`self.nPlayersInside`) (`self.nAlivePlayers`))
      (`self.OnPlayerEnter` self (`SphereComponent.SphereRadius` (`self.Sphere`))))))

(event `self.Sphere.OnComponentEndOverlap`
  (params (OverlappedComponent :type "PrimitiveComponent Object Reference") (OtherActor :type "Actor Object Reference") (OtherComp :type "PrimitiveComponent Object Reference") (OtherBodyIndex :type Integer))
  (if (`self.ActorHasTag` OtherActor "Player")
    (`self.DecrementPlayers`)
    (if (not (== (`self.nPlayersInside`) (`self.nAlivePlayers`)))
      (`self.OnPlayerExit` self (`SphereComponent.SphereRadius` (`self.Sphere`))))))

(fn `DecrementPlayers`
  (bind _result (`/Engine/EditorBlueprintResources/StandardMacros.DecrementInt` (`self.nPlayersInside`))
    (:`  `
      (if (< _result 0)
        (set `self.nPlayersInside` 0)))))

(fn `GetN_PlayersInside`
  (bind _returnvalue (`self.K2_GetActorLocation` self))
  (bind _outhits (`KismetSystemLibrary.SphereTraceMulti` _returnvalue _returnvalue (`SphereComponent.SphereRadius` (`self.Sphere`)) "TraceTypeQuery1"))
  (for _array_element _outhits
    (if (`.bInitialOverlap` (`GameplayStatics.BreakHitResult` _array_element))
      (if (`self.ActorHasTag` (`.HitActor` (`GameplayStatics.BreakHitResult` _array_element)) "Player")
        (`self.IncrementPlayers`)))))

(fn `IncrementPlayers`
  (bind _result (`/Engine/EditorBlueprintResources/StandardMacros.IncrementInt` (`self.nPlayersInside`))
    (:`  `
      (if (> _result (`self.nAlivePlayers`))
        (set `self.nPlayersInside` (`self.nAlivePlayers`))))))

(fn `Init`
  (params (nPlayers :type Integer) (zoneRadius :type "Float (double-precision)"))
  (bind _output_get (set `self.nAlivePlayers` nPlayers))
  (set `self.nPlayersInside` _output_get)
  (if (> zoneRadius 0.0)
    (`SphereComponent.SetSphereRadius` (`self.Sphere`) (* (`SphereComponent.SphereRadius` (`self.Sphere`)) zoneRadius) true)))

(fn `UpdatePlayerAlive`
  (params (nAlivePlayers :type Integer))
  (set `self.nAlivePlayers` nAlivePlayers))

(fn `UserConstructionScript`)