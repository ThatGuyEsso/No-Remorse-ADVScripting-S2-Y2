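; Shared multiplayer camera actor that adjusts its height to the spread of living players.
; Tick takes the farthest player's XY distance from the camera and interpolates Z toward a settings-based, clamped height.
; InitCamera also spawns concentric BP_CameraZoneTrigger zones with stepped radii.
; Their enter/exit zoom logic is left unbound because BindtoZones is empty, so only the distance-based zoom moves the camera after initialization.
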(event `Bind to Zones`
  ;[0 0 0] On Bind to Camera Zones(REDACTED)
)

(event `OnCharactersEnter`
  (params (zoneActor :type "/Game/Student/Blueprint/Gameplay/Camera/BP_CameraZoneTrigger Object Reference") (radius :type "Float (double-precision)"))
  ;[0 0 0] On Bind to Camera Zones(REDACTED)
  (bind _shouldzoom (`self.ShouldZoomIn` zoneActor))
  (if _shouldzoom
    (`self.ZoomIn` radius zoneActor)))

(event `OnCharacterExit`
  (params (ZoneActor :type "/Game/Student/Blueprint/Gameplay/Camera/BP_CameraZoneTrigger Object Reference") (radius :type "Float (double-precision)"))
  ;[0 0 0] On Bind to Camera Zones(REDACTED)
  (bind _shouldzoom (`self.ShouldZoomOut` ZoneActor))
  (if _shouldzoom
    (`self.ZoomOut` ZoneActor radius)))

(event `self.ReceiveTick`
  (params (DeltaSeconds :type "Float (single-precision)"))
  (bind (_returnvalue_x _returnvalue_y) (`KismetMathLibrary.BreakVector` (`self.K2_GetActorLocation`)))
  (bind (_returnvalue_x_2 _returnvalue_y_2 _returnvalue_z) (`KismetMathLibrary.BreakVector` (`self.K2_GetActorLocation`)))
  (bind (_camerasettings_minzoomin _camerasettings_maxzoomout _camerasettings_startingzoom _camerasettings_zoomspeed) (break `/Game/Student/Blueprint/Gameplay/Camera/S_CameraSettings` (`self.CameraSettings`)))
  ;[1 1 1] UpdateZoomHeight
  (bind _greatestdistance (`self.Evaluate Farthest Player`))
  (bind _output_get (set `self.targetHeight` (+ _camerasettings_startingzoom (* _greatestdistance 0.95))))
  (`self.K2_SetActorLocation` (`KismetMathLibrary.MakeVector` _returnvalue_x _returnvalue_y (`KismetMathLibrary.FInterpTo` _returnvalue_z (`KismetMathLibrary.FClamp` _output_get _camerasettings_minzoomin _camerasettings_maxzoomout) DeltaSeconds _camerasettings_zoomspeed))))

(fn `CreateCameraZones`
  (bind (_returnvalue_x _returnvalue_y) (`KismetMathLibrary.BreakVector` (`self.K2_GetActorLocation`)))
  (bind (_camerasettings_minzoomin _camerasettings_maxzoomout _camerasettings_startingzoom _camerasettings_zoomspeed _camerasettings_zonesizemultiplier _camerasettings_nzones) (break `/Game/Student/Blueprint/Gameplay/Camera/S_CameraSettings` (`self.CameraSettings`)))
  (bind (_camerasettings_minzoomin_2 _camerasettings_maxzoomout_2 _camerasettings_startingzoom_2 _camerasettings_zoomspeed_2 _camerasettings_zonesizemultiplier_2) (break `/Game/Student/Blueprint/Gameplay/Camera/S_CameraSettings` (`self.CameraSettings`)))
  (for _index (range _camerasettings_nzones)
    (bind _returnvalue (`|SpawnActorFromClass` "/Game/Student/Blueprint/Gameplay/Camera/BP_CameraZoneTrigger.BP_CameraZoneTrigger_C" (`KismetMathLibrary.MakeTransform` (`KismetMathLibrary.MakeVector` _returnvalue_x _returnvalue_y 150.0)) "AlwaysSpawn" "OverrideRootScale" null null))
    (`KismetArrayLibrary.Array_Add` (`self.Zones`) _returnvalue)
    (`/Game/Student/Blueprint/Gameplay/Camera/BP_CameraZoneTrigger.Init` _returnvalue (`KismetArrayLibrary.Array_Length` (`self.PlayerCharacters`)) (* _index _camerasettings_zonesizemultiplier_2)))
  (set `self.currentZone` (`|GetArrayItem` (`self.Zones`)))
  (`self.Bind to Zones`))

(fn `Evaluate Farthest Player`
  (returns (GreatestDistance :type "Float (double-precision)"))
  (locals (greatestOffset :type "Float (double-precision)" :default 0.0))
  (bind (_returnvalue_x _returnvalue_y) (`KismetMathLibrary.BreakVector` (`self.K2_GetActorLocation`)))
  (bind _players (message `/Game/Student/Blueprint/Interfaces/BPI_GameModeData.GetPlayersAlive` (`GameplayStatics.GetGameMode`)))
  (if (> (`KismetArrayLibrary.Array_Length` _players) 0)
    (for _array_element _players
      (bind (_returnvalue_x_2 _returnvalue_y_2) (`KismetMathLibrary.BreakVector` (`self.K2_GetActorLocation` _array_element)))
      (bind _returnvalue (`KismetMathLibrary.Distance2D` (`KismetMathLibrary.MakeVector2D` _returnvalue_x_2 _returnvalue_y_2) (`KismetMathLibrary.MakeVector2D` _returnvalue_x _returnvalue_y)))
      (if (> _returnvalue (`local.greatestOffset`))
        (set `local.greatestOffset` _returnvalue)))
    (return (`local.greatestOffset`))))

(fn `GetCamera`
  (returns (Camera :type "CameraComponent Object Reference"))
  (return (`self.Camera`)))

(fn `GetControllerRef`
  (returns (controllerRef :type "/Game/Student/Blueprint/Controllers/PC_ArenaController Object Reference"))
  (return null))

(fn `InitCamera`
  (params (CameraSettings :type "/Game/Student/Blueprint/Gameplay/Camera/S_CameraSettings Structure") (PlayerCharacters :type "Array of /Game/Student/Blueprint/Gameplay/Characters/BP_BaseTeamCharacter Object Reference"))
  (bind (_returnvalue_x _returnvalue_y) (`KismetMathLibrary.BreakVector` (`self.K2_GetActorLocation`)))
  (bind (_camerasettings_minzoomin _camerasettings_maxzoomout _camerasettings_startingzoom) (break `/Game/Student/Blueprint/Gameplay/Camera/S_CameraSettings` (`self.CameraSettings`)))
  (set `self.CameraSettings` CameraSettings)
  (set `self.PlayerCharacters` PlayerCharacters)
  (bind _output_get (set `self.targetHeight` _camerasettings_startingzoom))
  (`self.K2_SetActorLocation` (`KismetMathLibrary.MakeVector` _returnvalue_x _returnvalue_y _output_get))
  (bind _greatestdistance (`self.Evaluate Farthest Player`))
  (set `self.floatMaxStartingOffset` _greatestdistance)
  (`self.CreateCameraZones`))

(fn `ShouldZoomIn`
  (params (newZone :type "/Game/Student/Blueprint/Gameplay/Camera/BP_CameraZoneTrigger Object Reference"))
  (returns (shouldZoom :type Boolean))
  (locals (newIndex :type Integer :default 0))
  (bind _returnvalue (`KismetArrayLibrary.Array_Find` (`self.Zones`) (`self.currentZone`)))
  (bind _output_get (set `local.newIndex` (`KismetArrayLibrary.Array_Find` (`self.Zones`) newZone)))
  (if (<= _output_get _returnvalue)
    (set `self.zoneIndex` _output_get)
    (return true)
    (else
      (set `self.zoneIndex` _returnvalue)
      (return false))))

(fn `ShouldZoomOut`
  (params (newZone :type "/Game/Student/Blueprint/Gameplay/Camera/BP_CameraZoneTrigger Object Reference"))
  (returns (shouldZoom :type Boolean))
  (locals (newIndex :type Integer :default 0))
  (bind _returnvalue (`KismetArrayLibrary.Array_Find` (`self.Zones`) (`self.currentZone`)))
  (bind _output_get (set `local.newIndex` (`KismetArrayLibrary.Array_Find` (`self.Zones`) newZone)))
  (if (>= _output_get _returnvalue)
    (set `self.zoneIndex` _output_get)
    (return true)
    (else
      (set `self.zoneIndex` _returnvalue)
      (return false))))

(fn `UpdateAlivePlayers`
  (params (playerAlive :type Integer))
  (for _array_element (`self.Zones`)
    (`/Game/Student/Blueprint/Gameplay/Camera/BP_CameraZoneTrigger.UpdatePlayerAlive` _array_element playerAlive)))

(fn `UserConstructionScript`)

(fn `ZoomIn`
  (params (radius :type "Float (double-precision)") (currentZone :type "/Game/Student/Blueprint/Gameplay/Camera/BP_CameraZoneTrigger Object Reference"))
  (bind (_returnvalue_x _returnvalue_y _returnvalue_z) (`KismetMathLibrary.BreakVector` (`self.K2_GetActorLocation`)))
  (bind (_returnvalue_x_2 _returnvalue_y_2 _returnvalue_z_2) (`KismetMathLibrary.BreakVector` (`self.K2_GetActorLocation`)))
  (bind _camerasettings_minzoomin (break `/Game/Student/Blueprint/Gameplay/Camera/S_CameraSettings` (`self.CameraSettings`)))
  (bind _returnvalue (- _returnvalue_z radius))
  (set `self.currentZone` currentZone)
  (if (== (`self.zoneIndex`) (`KismetArrayLibrary.Array_LastIndex` (`self.Zones`)))
    ;[1 1 1] Adjust Zoom Intesnsity for the most outside zone
    (bind _output_get (set `self.targetHeight` (* _returnvalue 1.75)))
    ;[1 1 1] Evaluate whether the min zoom is greater than the minimun zoom intensity.
    (if (< _output_get _camerasettings_minzoomin)
      (set `self.targetHeight` _camerasettings_minzoomin :!label _label)
      ;[1 1 1] If not at desired height move camerea
      (if (!= (stale _output_get_2) _returnvalue_z_2) :!label _label_2
        (set `self.isMoving` true)
        (else
          (set `self.isMoving` false))))
    (else
      (bind _output_get_2 (set `self.targetHeight` _returnvalue))
      (if (< _output_get_2 _camerasettings_minzoomin)
        (goto _label)
        (else
          (goto _label_2))))))

(fn `ZoomOut`
  (params (currentZone :type "/Game/Student/Blueprint/Gameplay/Camera/BP_CameraZoneTrigger Object Reference") (radius :type "Float (double-precision)"))
  (bind (_returnvalue_x _returnvalue_y _returnvalue_z) (`KismetMathLibrary.BreakVector` (`self.K2_GetActorLocation`)))
  (bind (_camerasettings_minzoomin _camerasettings_maxzoomout _camerasettings_startingzoom) (break `/Game/Student/Blueprint/Gameplay/Camera/S_CameraSettings` (`self.CameraSettings`)))
  (set `self.currentZone` currentZone)
  (bind _output_get (set `self.targetHeight` (+ _camerasettings_startingzoom radius)))
  (if (> (`self.targetHeight`) _camerasettings_maxzoomout)
    (set `self.targetHeight` _camerasettings_maxzoomout))
  (if (!= _output_get _returnvalue_z)
    (set `self.isMoving` true)
    (else
      (set `self.isMoving` false))))