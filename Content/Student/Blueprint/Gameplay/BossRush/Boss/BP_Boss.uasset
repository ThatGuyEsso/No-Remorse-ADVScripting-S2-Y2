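; Boss-rush boss character that starts when the game mode signals Game Running, setting up its health bar and AIC_Boss controller.
; Timers alternate Idle and Attack states, randomly picking fast or slow spinning projectile volleys or spinning charges.
; Tick eases spin speed, while charges line-trace toward a living player and timeline-lerp there, damaging players hit.
; Damage grants flashing invulnerability and attacker score; death darkens and sinks the boss, then ends the game.
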(event `/Game/Student/Blueprint/Interfaces/BPI_Init.InitActor`
  ;[1 1 1] On Init
  (bind _zombiegamemode (message `/Game/Student/Blueprint/Interfaces/BPI_ZombieSurvival.GetGameModeRef` (`GameplayStatics.GetGameMode`)))
  (add `/Game/Student/Blueprint/GameModes/GM_ZombieSurvial.OnNewState` _zombiegamemode (delegate `OnNewGameState`)))

(event `OnNewGameState`
  (params (newState :type "/Game/Student/Blueprint/Data/E_GameStates Enum" :default "NewEnumerator0"))
  ;[1 1 1] On Init
  (switch `/Game/Student/Blueprint/Data/E_GameStates` newState
    (:`NewEnumerator5`
      (set `self.IsGameRunning` true)
      (`self.Init`)
      (set `self.origin` (`self.K2_GetActorLocation`))
      (set `self.currentHealth` (`self.MaxHealth`))
      (`self.SetUpUI`))))

(event `BeginBossBattle`
  ;[1 1 1] Begin Boss Battle
  (`self.SetNewState` "NewEnumerator0")
  (`KismetSystemLibrary.Delay` (`KismetMathLibrary.RandomFloatInRange` 3.0 5.0))
  (`self.GetRandomPlayer`)
  (`self.GetNewAttackType`)
  (`self.SetNewState` "NewEnumerator2")
  (`self.OnAttackCounter`))

(event `OnAttackCounter`
  ;[1 1 1] Attack duration and Cooldown
  (`KismetSystemLibrary.Delay` (`KismetMathLibrary.RandomFloatInRange` (`self.MinAttackDuration`) (`self.MaxAttackDuration`)))
  (`self.SetNewState` "NewEnumerator0")
  (set `self.CurrentAttackPattern` "NewEnumerator3")
  (`self.OnBeginAttackCounter`)
  (set `self.IsShooting` false))

(event `/Game/Student/Blueprint/Gameplay/BossRush/Boss/BPI_Boss.UpdateBossState`
  (params (NewState :type "/Game/Student/Blueprint/Gameplay/BossRush/Boss/E_BossState Enum" :default "NewEnumerator0"))
  (`self.SetNewState` NewState))

(event `OnBeginAttackCounter`
  ;[1 1 1] Attack duration and Cooldown
  (`KismetSystemLibrary.Delay` (`KismetMathLibrary.RandomFloatInRange` (`self.minAttackCoooldown`) (`self.maxAttackCooldown`)))
  (`self.GetRandomPlayer`)
  (`self.GetNewAttackType`)
  (`self.SetNewState` "NewEnumerator2")
  (`self.OnAttackCounter`))

(event `ShootLoop`
  ;[1 1 1] Shoot Loop
  (if (and (`self.IsShooting`) (!= (`self.dead`) true))
    (switch `/Game/Student/Blueprint/Gameplay/BossRush/Boss/E_AttackTypes` (`self.CurrentAttackPattern`)
      (:`NewEnumerator0`
        _)
      (:`NewEnumerator2`
        _))
    (`self.Shoot`)
    (`KismetSystemLibrary.Delay` (`self.fireRate`))
    (`self.ShootLoop`)))

(event `ChargeLoop`
  ;[1 1 1] Charging Loop
  (if (not (`self.IsCharging`))
    (switch `/Game/Student/Blueprint/Gameplay/BossRush/Boss/E_AttackTypes` (`self.CurrentAttackPattern`)
      (:`NewEnumerator1`
        (`self.OnCharge`)
        (`KismetSystemLibrary.Delay` 5.0)
        (bind (_nonealive _player) (`self.GetRandomAliveplayer`))
        (if _nonealive
          (set `self.CurrentTarget` _player)
          (`self.ChargeLoop`)
          (else
            (`self.SetNewState` "NewEnumerator0")))))))

(event `self.ReceiveTick`
  (params (DeltaSeconds :type "Float (single-precision)"))
  (bind (_returnvalue_roll _returnvalue_pitch _returnvalue_yaw) (`KismetMathLibrary.BreakRotator` (`self.K2_GetActorRotation`)))
  (if (not (`self.dead`))
    (set `self.deltaTime` DeltaSeconds)
    (switch `/Game/Student/Blueprint/Gameplay/BossRush/Boss/E_AttackTypes` (`self.CurrentAttackPattern`)
      (:`NewEnumerator0`
        _)
      (:`NewEnumerator1`
        _)
      (:`NewEnumerator2`
        _))
    (`self.K2_SetActorRotation` (`KismetMathLibrary.MakeRotator` _returnvalue_roll _returnvalue_pitch (+ _returnvalue_yaw (* (`self.deltaTime`) (`self.currentSpinSpeed`)))))
    (set `self.currentSpinSpeed` (`KismetMathLibrary.FInterpTo` (`self.currentSpinSpeed`) (`self.maxSpinSpeed`) (`self.deltaTime`) (`self.SpinAcceleration`)))))

(event `OnCharge`
  (bind (_returnvalue_x _returnvalue_y _returnvalue_z) (`KismetMathLibrary.BreakVector` (`self.K2_GetActorLocation`)))
  (bind _returnvalue (`self.K2_GetActorLocation`))
  (bind (_returnvalue_x_2 _returnvalue_y_2) (`KismetMathLibrary.BreakVector` (* (`KismetMathLibrary.GetDirectionUnitVector` (`self.K2_GetActorLocation`) (`self.K2_GetActorLocation` (`self.CurrentTarget`))) (`self.chargeDistance`))))
  (bind _output_get (set `self.ChargeTarget` (`KismetMathLibrary.MakeVector` _returnvalue_x_2 _returnvalue_y_2 _returnvalue_z)))
  (bind (_outhit _returnvalue_2) (`KismetSystemLibrary.LineTraceSingle` :`Start` _returnvalue :`End` (+ _returnvalue _output_get) :`TraceChannel` "TraceTypeQuery1" :`DrawDebugType` "ForDuration" :`DrawTime` 2.0))
  (if _returnvalue_2
    (set `self.ChargeTarget` (`.ImpactPoint` (`GameplayStatics.BreakHitResult` _outhit)))
    (else
      (set `self.ChargeTarget` (+ (`self.K2_GetActorLocation`) (`self.ChargeTarget`)))))
  (set `self.IsCharging` true)
  (bind (_direction _chargetime) (`Timeline|ChargeTimeLine` :!via `PlayFromStart` :!label _label)
    (:`Update`
      (`self.K2_SetActorLocation` (`KismetMathLibrary.VLerp` (`self.K2_GetActorLocation`) (`self.ChargeTarget`) _chargetime) true))
    (:`Finished`
      (set `self.IsCharging` false))))

(event `OnStopCharge`
  (goto _label :!via `Stop`))

(event `self.Collider.OnComponentHit`
  (params (HitComponent :type "PrimitiveComponent Object Reference") (OtherActor :type "Actor Object Reference") (OtherComp :type "PrimitiveComponent Object Reference") (NormalImpulse :type "Vector Structure") (Hit :type "HitResult Structure (by ref)"))
  (bind (_returnvalue_x _returnvalue_y) (`KismetMathLibrary.BreakVector` (`KismetMathLibrary.Normal` (`self.GetVelocity`))))
  (if (`self.IsCharging`)
    (if (`self.ActorHasTag` OtherActor "Player")
      (message `/Game/Student/Blueprint/Gameplay/Characters/Interfaces/BPI_Hurtable.DamageActor` OtherActor self (`self.ChargeDamage`) (`self.knockBack`) (`KismetMathLibrary.MakeVector` _returnvalue_x _returnvalue_y))
      (`self.OnStopCharge`)
      (`KismetSystemLibrary.Delay` 2.0)
      (set `self.IsCharging` false))))

(event `/Game/Student/Blueprint/Gameplay/Characters/Interfaces/BPI_Hurtable.DamageActor`
  (params (InterfaceActor :type "Actor Object Reference") (dmg :type "Float (single-precision)") (knockBack :type "Float (single-precision)") (KnockBarDir :type "Vector Structure"))
  (bind _returnvalue (- (`self.currentHealth`) dmg))
  (if (`self.isHurt`)
    _
    (elif (not (`self.dead`))
      (`self.PlayHurtSFX`)
      (if (<= _returnvalue 0.0)
        (set `self.dead` true)
        (bind _output_get (set `self.currentHealth` 0.0))
        (`/Game/Student/Blueprint/Widgets/BPW_BossHealth.UpdateHealth` (`self.BossHealthBar`) _output_get (`self.MaxHealth`))
        (`self.OnBossDefeated`)
        (`self.BossDefeated`)
        (else
          (set `self.currentHealth` _returnvalue)
          (message `/Game/Student/Blueprint/Gameplay/Characters/Interfaces/BPI_Scoreable.AddScore` (`self.GetOwner` InterfaceActor) (`KismetMathLibrary.FTrunc` dmg) null)
          (set `self.isHurt` true)
          (`self.OnHurt`)
          (`/Game/Student/Blueprint/Widgets/BPW_BossHealth.UpdateHealth` (`self.BossHealthBar`) (`self.currentHealth`) (`self.MaxHealth`)))))))

(event `OnHurt`
  (`self.FlashOn`)
  (`KismetSystemLibrary.Delay` (`self.hurtTime`))
  (set `self.isHurt` false)
  (`self.SetDefaultMat`))

(event `FlashOn`
  ;[1 1 1] If is hurt
  (if (`self.isHurt`)
    ;[1 1 1] Change to hurt mat
    (`self.SetHurtMat`)
    (`KismetSystemLibrary.Delay` (`self.flashRate`))
    (`self.FlashOff`)
    (else
      ;[1 1 1] switch to not hurt mat
      (`self.SetDefaultMat`))))

(event `FlashOff`
  ;[1 1 1] If is hurt
  (if (`self.isHurt`)
    ;[1 1 1] Go to default mat then prepare to flash on
    (`self.SetDefaultMat`)
    (`KismetSystemLibrary.Delay` (`self.flashRate`))
    (`self.FlashOn`)
    (else
      ;[1 1 1] Go to default mat
      (`self.SetHurtMat`))))

(event `BossDefeated`
  (bind (_returnvalue_x _returnvalue_y _returnvalue_z) (`KismetMathLibrary.BreakVector` (`self.K2_GetActorLocation`)))
  (`self.SetDeathMath`)
  (set `CharacterMovementComponent.MaxWalkSpeed` 0.0 (`self.CharacterMovement`))
  (set `self.deathPos` (`KismetMathLibrary.MakeVector` _returnvalue_x _returnvalue_y (- _returnvalue_z 40.0)))
  (bind (_direction _deathlerp) (`Timeline|DeathTimeLine` :!via `PlayFromStart`)
    (:`Update`
      (`self.K2_SetActorLocation` (`KismetMathLibrary.VLerp` (`self.K2_GetActorLocation`) (`self.deathPos`) _deathlerp)))
    (:`Finished`
      (message `/Game/Student/Blueprint/Interfaces/BPI_ZombieSurvival.BeginEndGame` (`GameplayStatics.GetGameMode`)))))

(fn `EvaluateNewAttackType`
  (if (not (or (`self.IsCharging`) (`self.IsShooting`)))
    (switch `/Game/Student/Blueprint/Gameplay/BossRush/Boss/E_AttackTypes` (`self.CurrentAttackPattern`)
      (:`NewEnumerator0`
        (`self.InitSpinShot`))
      (:`NewEnumerator1`
        (`self.InitSpinCharge`))
      (:`NewEnumerator2`
        (`self.InitSlowSpinShoot`))
      (:`NewEnumerator3`
        (set `self.IsShooting` false)
        (set `self.IsCharging` false)))))

(fn `EvaluateNewState`
  (switch `/Game/Student/Blueprint/Gameplay/BossRush/Boss/E_BossState` (`self.currentState`)
    (:`NewEnumerator2`
      (`self.EvaluateNewAttackType`))))

(fn `GetBossData`
  (returns (DefaultState :type "/Game/Student/Blueprint/Gameplay/BossRush/Boss/E_BossState Enum") (CurrentState :type "/Game/Student/Blueprint/Gameplay/BossRush/Boss/E_BossState Enum") (AttackRange :type "Float (double-precision)") (currentTarget :type "Actor Object Reference"))
  (return (`self.DefaultState`) (`self.currentState`) (`self.AttackRange`) (`self.CurrentTarget`)))

(fn `GetClosesPlayer`)

(fn `GetMapOrigin`
  (returns (MapOrigin :type "Vector Structure"))
  (return (`self.origin`)))

(fn `GetNewAttackType`
  (set `self.CurrentAttackPattern` (cast `/Game/Student/Blueprint/Gameplay/BossRush/Boss/E_AttackTypes` (`KismetMathLibrary.Conv_IntToByte` (`KismetMathLibrary.RandomInteger` 3)))))

(fn `GetRandomAliveplayer`
  (returns (NoneAlive :type Boolean) (player :type "/Game/Student/Blueprint/Gameplay/Characters/BP_BaseTeamCharacter Object Reference"))
  (locals (AlivePlayers :type "Array of /Game/Student/Blueprint/Gameplay/Characters/BP_BaseTeamCharacter Object Reference"))
  (bind _players (message `/Game/Student/Blueprint/Interfaces/BPI_GameModeData.GetPlayersAlive` (`GameplayStatics.GetGameMode`)))
  (bind _output_get (set `local.AlivePlayers` _players))
  (if (> (`KismetArrayLibrary.Array_Length` _output_get) 0)
    (return true (`|GetArrayItem` _output_get (`KismetMathLibrary.RandomInteger` (`KismetArrayLibrary.Array_Length` _output_get))))
    (else
      (return false null))))

(fn `GetRandomPlayer`
  (returns (Player :type "/Game/Student/Blueprint/Gameplay/Characters/BP_BaseTeamCharacter Object Reference") (PlayerFound :type Boolean))
  (bind _players (`self.players`))
  (if (> (`KismetArrayLibrary.Array_Length` (`self.players`)) 0)
    (return (`|GetArrayItem` _players (`KismetMathLibrary.RandomInteger` (`KismetArrayLibrary.Array_Length` _players))) true)
    (else
      (return null false))))

(fn `GetTeam`
  (returns (Team :type "/Game/Student/Blueprint/Data/E_Teams Enum"))
  (return "NewEnumerator3"))

(fn `Init`
  (bind _characterlights (`self.characterLights`))
  (bind _players (message `/Game/Student/Blueprint/Interfaces/BPI_GameModeData.GetPlayers` (`GameplayStatics.GetGameMode`)))
  (set `self.players` _players)
  (bind (_player _playerfound) (`self.GetRandomPlayer`))
  (if _playerfound
    (set `self.CurrentTarget` _player)
    (bind _asaic_boss (cast `/Game/Student/Blueprint/Controllers/AIC_Boss` (`self.GetController`)))
    (`/Game/Student/Blueprint/Controllers/AIC_Boss.Init` _asaic_boss)
    (`KismetArrayLibrary.Array_Add` (`self.FirePoints`) (`self.ShootDirection`))
    (`KismetArrayLibrary.Array_Add` (`self.FirePoints`) (`self.ShootDirection1`))
    (`KismetArrayLibrary.Array_Add` (`self.FirePoints`) (`self.ShootDirection2`))
    (`KismetArrayLibrary.Array_Add` (`self.FirePoints`) (`self.ShootDirection3`))
    (`KismetArrayLibrary.Array_Add` (`self.characterLights`) (`self.RimLight`))
    (`KismetArrayLibrary.Array_Add` _characterlights (`self.RimlightTop`))
    (`KismetArrayLibrary.Array_Add` _characterlights (`self.RimlightTop1`))
    (`self.BeginBossBattle`)))

(fn `InitSlowSpinShoot`
  (set `self.AttackRange` 2000.0)
  (set `self.currentSpinSpeed` 0.0)
  (set `self.maxSpinSpeed` 100.0)
  (set `self.fireRate` 0.1)
  (set `self.IsShooting` true)
  (`self.ShootLoop`))

(fn `InitSpinCharge`
  (if (not (`self.IsCharging`))
    (set `self.AttackRange` 2000.0)
    (set `self.currentSpinSpeed` 0.0)
    (set `self.maxSpinSpeed` 600.0)
    (`self.ChargeLoop`)))

(fn `InitSpinShot`
  (set `self.AttackRange` 2000.0)
  (set `self.currentSpinSpeed` 0.0)
  (set `self.maxSpinSpeed` 400.0)
  (set `self.fireRate` 0.25)
  (set `self.IsShooting` true)
  (`self.ShootLoop`))

(fn `IsOnTeam`
  (params (CallerTeam :type "/Game/Student/Blueprint/Data/E_Teams Enum" :default "NewEnumerator0"))
  (returns (IsOnTeam :type Boolean))
  (return false))

(fn `PlayHurtSFX`
  (`GameplayStatics.PlaySoundAtLocation` "/Game/Student/Assets/SFX/bossHurt.BossHurt" (`self.K2_GetActorLocation`) (struct) 1.0 (`KismetMathLibrary.RandomFloatInRange` 0.8 1.2) 0.0 null null null))

(fn `SetDeathMath`
  (for _array_element (`self.characterLights`)
    (bind _returnvalue (`PrimitiveComponent.CreateDynamicMaterialInstance` _array_element 0 (`PrimitiveComponent.GetMaterial` _array_element 0) "None"))
    (`MaterialInstanceDynamic.SetVectorParameterValue` _returnvalue "tint" (struct :`A` 1.0))))

(fn `SetDefaultMat`
  (for _array_element (`self.characterLights`)
    (bind _returnvalue (`PrimitiveComponent.CreateDynamicMaterialInstance` _array_element 0 (`PrimitiveComponent.GetMaterial` _array_element 0) "None"))
    (`MaterialInstanceDynamic.SetVectorParameterValue` _returnvalue "tint" (struct :`R` 1.0 :`G` 0.07451 :`B` 0.090196 :`A` 1.0))))

(fn `SetHurtMat`
  (for _array_element (`self.characterLights`)
    (bind _returnvalue (`PrimitiveComponent.CreateDynamicMaterialInstance` _array_element 0 (`PrimitiveComponent.GetMaterial` _array_element 0) "None"))
    (`MaterialInstanceDynamic.SetVectorParameterValue` _returnvalue "tint" (struct :`R` 1.0 :`G` 1.0 :`B` 1.0 :`A` 1.0))))

(fn `SetNewState`
  (params (currentState :type "/Game/Student/Blueprint/Gameplay/BossRush/Boss/E_BossState Enum" :default "NewEnumerator0"))
  (bind _output_get (set `self.currentState` currentState))
  (`self.EvaluateNewState`)
  (`self.OnStateChange` _output_get))

(fn `SetUpUI`
  (bind _returnvalue (`|CreateWidget` "/Game/Student/Blueprint/Widgets/BPW_BossHealth.BPW_BossHealth_C"))
  (bind _output_get (set `self.BossHealthBar` _returnvalue))
  (`UserWidget.AddToViewport` _output_get 1)
  (`/Game/Student/Blueprint/Widgets/BPW_BossHealth.SetUpHealth` _output_get))

(fn `Shoot`
  (for _array_element (`self.FirePoints`)
    (bind _team (message `/Game/Student/Blueprint/Interfaces/BPI_TeamData.GetTeam` self))
    (bind _returnvalue (`SceneComponent.GetForwardVector` _array_element))
    (`|SpawnActorFromClass` "/Game/Student/Blueprint/Gameplay/Weapons/BP_TeamProjectile.BP_TeamProjectile_C" (`KismetMathLibrary.MakeTransform` (+ _returnvalue (`SceneComponent.K2_GetComponentLocation` _array_element)) (`KismetMathLibrary.MakeRotFromX` _returnvalue)) "AlwaysSpawn" "OverrideRootScale" null _team (struct :`R` 1.0 :`G` 0.818793 :`B` 0.38212 :`A` 1.0) (`self.projectileDamage`) null))
  (`GameplayStatics.PlaySoundAtLocation` "/Game/Audio/TwinStickFire.TwinStickFire" (`self.K2_GetActorLocation`) (struct) 0.5 1.0 0.0 null null null))

(fn `UserConstructionScript`)