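; Base team character for an arena game, adding launch-based jumping and dashing, team identity and score tracking.
; Jump and dash use LaunchCharacter with limited charges; jumps reset on landing, dashes on a cooldown timer, and gravity increases while falling.
; In Zombie Survival, Init waits for the game mode's Game Running state to set up movement and weapon UI.
; Team assignment picks armour colour, and score is forwarded to the controller.
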(event `GetComponentRefs`
  ;[1 1 1] Getting Components
  (bind _aspc_arena_controller (cast `/Game/Student/Blueprint/Controllers/PC_ArenaController` (`self.GetController`)))
  (set `self.controllerRef` _aspc_arena_controller))

(event `/Game/Student/Blueprint/Gameplay/Characters/Interfaces/BPI_CharacterActions.OnJump`
  ;[1 1 1] On Jump
  (if (> (`self.nJumps`) 0)
    (if (`self.IsGrounded`)
      (`self.DoJump`))))

(event `/Game/Student/Blueprint/Gameplay/Characters/Interfaces/BPI_CharacterActions.OnDash`
  ;[1 1 1] On Dash
  (if (> (`self.nDashes`) 0)
    (`self.DoDash`)
    (elif (not (`self.IsDashRefeshing`))
      (bind _returnvalue (`KismetSystemLibrary.K2_SetTimer` null "RefreshDash" (`self.DashCoolDown`)))
      (set `self.DashCooldownHandle` _returnvalue)
      (set `self.IsDashRefeshing` true))))

(event `self.OnLaunched`
  (params (LaunchVelocity :type "Vector Structure") (bXYOverride :type Boolean) (bZOverride :type Boolean))
  ;[1 1 1] On Launched
  (set `self.IsGrounded` false))

(event `self.OnLanded`
  (params (Hit :type "HitResult Structure (by ref)"))
  ;[1 1 1] On Landed
  (set `self.nJumps` (`self.MaxJumps`))
  (set `CharacterMovementComponent.GravityScale` (`self.defaultGravity`) (`self.CharacterMovement`))
  (set `self.IsGrounded` true))

(event `self.ReceiveTick`
  (params (DeltaSeconds :type "Float (single-precision)"))
  ;[1 1 1] On Tick
  (`|ExecutionSequence`
    (:`then_0`
      (if (`NavMovementComponent.IsFalling` (`self.CharacterMovement`))
        (set `CharacterMovementComponent.GravityScale` (* (`self.defaultGravity`) (`self.gravityMultiplier`)) (`self.CharacterMovement`))))))

(event `/Game/Student/Blueprint/Interfaces/BPI_Init.InitActor`
  ;[1 1 1] On Init
  (bind _gamemodetype (message `/Game/Student/Blueprint/Interfaces/BPI_GameModeData.GetGameType` (`GameplayStatics.GetGameMode`)))
  (switch `/Game/Student/Blueprint/Data/E_GameModes` _gamemodetype
    (:`NewEnumerator0`
      (bind _zombiegamemode (message `/Game/Student/Blueprint/Interfaces/BPI_ZombieSurvival.GetZombieGameModeRef` (`GameplayStatics.GetGameMode`)))
      (add `/Game/Student/Blueprint/GameModes/GM_ZombieSurvial.OnNewState` _zombiegamemode (delegate `OnNewStae`)))))

(event `OnNewStae`
  (params (newState :type "/Game/Student/Blueprint/Data/E_GameStates Enum" :default "NewEnumerator0"))
  ;[1 1 1] On Init
  (switch `/Game/Student/Blueprint/Data/E_GameStates` newState
    (:`NewEnumerator5`
      (`self.Init`))))

(event `/Game/Student/Blueprint/Interfaces/BPI_TeamData.AssignTeam`
  (params (Team :type "/Game/Student/Blueprint/Data/E_Teams Enum" :default "NewEnumerator0"))
  ;[1 1 1] On assign character's team
  (set `self.Team` Team)
  (`self.EvaluateTeam`))

(event `/Game/Student/Blueprint/Gameplay/Characters/Interfaces/BPI_Scoreable.AddScore`
  (params (Score :type Integer) (Player :type "Actor Object Reference"))
  (bind _output_get (set `self.currentScore` (+ Score (`self.currentScore`))))
  (message `/Game/Student/Blueprint/Widgets/Interfaces/BPI_ScoreWidget.SetScore` (`self.GetController`) _output_get))

(fn `DoDash`
  (if (`NavMovementComponent.IsFalling` (`self.CharacterMovement`))
    (if (!= (`PawnMovementComponent.GetLastInputVector` (`self.CharacterMovement`)) (0.0 0.0 0.0))
      (`self.LaunchCharacter` (* (`PawnMovementComponent.GetLastInputVector` (`self.CharacterMovement`)) (`self.DashForceAir`)))
      (else
        (`self.LaunchCharacter` (* (`self.GetActorForwardVector`) (`self.DashForceAir`)))))
    (elif (!= (`PawnMovementComponent.GetLastInputVector` (`self.CharacterMovement`)) (0.0 0.0 0.0))
      (`self.LaunchCharacter` (* (`PawnMovementComponent.GetLastInputVector` (`self.CharacterMovement`)) (`self.DashForce`)))
      (else
        (`self.LaunchCharacter` (* (`self.GetActorForwardVector`) (`self.DashForce`))))))
  (`/Engine/EditorBlueprintResources/StandardMacros.DecrementInt` (`self.nDashes`)
    (:`  `
      (if (<= (`self.nDashes`) 0)
        (bind _returnvalue (`KismetSystemLibrary.K2_SetTimer` null "RefreshDash" (`self.DashCoolDown`)))
        (set `self.DashCooldownHandle` _returnvalue)
        (set `self.IsDashRefeshing` true)))))

(fn `DoJump`
  (`self.LaunchCharacter` (* (`self.GetActorUpVector`) (`self.JumpForce`)))
  (`/Engine/EditorBlueprintResources/StandardMacros.DecrementInt` (`self.nJumps`)))

(fn `EvaluateTeam`
  (switch `/Game/Student/Blueprint/Data/E_Teams` (`self.Team`)
    (:`NewEnumerator0`
      (set `self.ArmourColour` (struct :`R` 0.725632 :`G` 0.070355 :`B` 1.0 :`A` 1.0)))
    (:`NewEnumerator1`
      (set `self.ArmourColour` (struct :`G` 1.0 :`B` 0.084535 :`A` 1.0)))
    (:`NewEnumerator2`
      (set `self.ArmourColour` (struct :`R` 0.123748 :`G` 0.224498 :`B` 0.675 :`A` 1.0)))))

(fn `GetControllerRef`
  (returns (controllerRef :type "/Game/Student/Blueprint/Controllers/PC_ArenaController Object Reference"))
  (return (`self.controllerRef`)))

(fn `GetGameType`
  (returns (GameModeType :type "/Game/Student/Blueprint/Data/E_GameModes Enum"))
  (return "NewEnumerator0"))

(fn `GetIsAlive`
  (returns (ISAlive :type Boolean))
  (if (`self.dead`)
    (return false)
    (else
      (return true))))

(fn `GetPlayers`
  (returns (Players :type "Array of /Game/Student/Blueprint/Gameplay/Characters/BP_BaseTeamCharacter Object Reference"))
  (return))

(fn `GetTeam`
  (returns (Team :type "/Game/Student/Blueprint/Data/E_Teams Enum"))
  (return (`self.Team`)))

(fn `GetZombieGameModeRef`
  (returns (ZombieGameMode :type "/Game/Student/Blueprint/GameModes/GM_ZombieSurvial Object Reference"))
  (return null))

(fn `Init`
  (set `CharacterMovementComponent.AirControl` (`self.DefaultAirControl`) (`self.CharacterMovement`))
  (set `self.nJumps` (`self.MaxJumps`))
  (set `self.nDashes` (`self.MaxDashes`))
  (`PrimitiveComponent.SetCastShadow` (`self.WeaponWidget`) false)
  (`/Game/Framework_Blueprints/UI/PlayerWeaponUI.Init` (cast `/Game/Framework_Blueprints/UI/PlayerWeaponUI` (`WidgetComponent.GetUserWidgetObject` (`self.WeaponWidget`)) :!pure true) self)
  (`parent.Init`))

(fn `IsAtZombieCapacity`
  (returns (IsAtCapacity :type Boolean))
  (return false))

(fn `IsOnTeam`
  (params (CallerTeam :type "/Game/Student/Blueprint/Data/E_Teams Enum" :default "NewEnumerator0"))
  (returns (IsOnTeam :type Boolean))
  (return (== CallerTeam (`self.Team`))))

(fn `RefreshDash`
  (set `self.nDashes` (`self.MaxDashes`))
  (set `self.IsDashRefeshing` false))

(fn `UserConstructionScript`
  (`parent.UserConstructionScript`))