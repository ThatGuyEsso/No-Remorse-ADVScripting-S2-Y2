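; Zombie enemy character that chases and melees players, with stats read from AIData.
; An Idle/Chase/Attack state switch sets movement and cooldown-gated attack montages, whose events trigger team-filtered damage through collision overlap and a sphere trace.
; Damage starts a timed invulnerability with material flashing; death awards score, notifies game mode and controller, and later sinks the body before destroying it.
; Targets come from capsule hits, or the nearest living player when the current target dies.
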(event `self.ReceiveBeginPlay`
  (`PrimitiveComponent.SetCollisionEnabled` (`self.attackCollison`) "NoCollision"))

(event `/Game/Student/Blueprint/Gameplay/Characters/Interfaces/BPI_Zombie.UpdateZombieState`
  (params (NewState :type "/Game/Student/Blueprint/Gameplay/ZombieSurvival/AI/Data/E_ZombieStates Enum" :default "NewEnumerator0"))
  (`self.SetNewState` NewState))

(event `/Game/Student/Blueprint/Gameplay/Characters/Interfaces/BPI_Hurtable.DamageActor`
  (params (InterfaceActor :type "Actor Object Reference") (dmg :type "Float (single-precision)") (knockBack :type "Float (single-precision)") (KnockBarDir :type "Vector Structure"))
  ;[1 1 1] Is it still on  cool down
  (if (`self.CanBehurt`)
    ;[1 1 1] Does it have any remaining health
    (bind _output_get (set `self.currentHealth` (- (`self.currentHealth`) dmg)))
    (if (<= _output_get 0.0)
      ;[1 1 1] If no health, add points to player that fired the killing shot
      (message `/Game/Student/Blueprint/Gameplay/Characters/Interfaces/BPI_Hurtable.DamageActorDied` InterfaceActor self)
      (message `/Game/Student/Blueprint/Interfaces/BPI_ZombieSurvival.ZombieKilled` (`GameplayStatics.GetGameMode`))
      (if (not (`self.isDead`))
        (message `/Game/Student/Blueprint/Gameplay/Characters/Interfaces/BPI_Scoreable.AddScore` (`self.GetOwner` InterfaceActor) 10 null)
        ;[1 1 1] become idle and begin death montage + death events
        (set `self.isDead` true)
        (`self.SetNewState` "NewEnumerator0")
        (`|PlayMontage` (`self.Mesh`) "/Game/Student/Assets/Animation/Zombie/M_ZombieDeath.M_ZombieDeath"
          (:`then`
            (message `/Game/Student/Blueprint/Gameplay/Characters/Interfaces/BPI_Zombie.BeginDeath` (`self.GetController`))
            ;[1 1 1] Disable collision
            (`PrimitiveComponent.SetCollisionEnabled` (`self.CapsuleComponent`) "NoCollision"))))
      (else
        ;[1 1 1] If yes start hurt time
        (set `self.CanBehurt` false)
        (`self.StartHurtTime`)
        (`self.FlashOn`)))))

(event `/Game/Student/Blueprint/Gameplay/Characters/Interfaces/BPI_Zombie.Died`
  ;[1 1 1] On death
  ;[1 1 1] Wait a for some time then begin to hide characters body
  (`KismetSystemLibrary.Delay` (`KismetMathLibrary.RandomFloatInRange` (`self.minDeathHideDelay`) (`self.maxDeathHideDelay`)))
  (`self.BeginToHideZombieBody`))

(event `BeginToHideZombieBody`
  (bind (_returnvalue_x _returnvalue_y _returnvalue_z) (`KismetMathLibrary.BreakVector` (`self.K2_GetActorLocation`)))
  (bind (_returnvalue_x_2 _returnvalue_y_2 _returnvalue_z_2) (`KismetMathLibrary.BreakVector` (`self.K2_GetActorLocation`)))
  ;[1 1 1] On begin to hide zombie body
  ;;[1 0.9894 0.4859] Get current actor z Position
  (set `self.actorZ` _returnvalue_z)
  ;;[1 0.9157 0.33] Lerp actor until z position is equal to desired. Then destroy actor
  (bind (_direction _hidealpha) (`Timeline|hidingTimline` :!via `PlayFromStart`)
    (:`Update`
      (`self.K2_SetActorLocation` (`KismetMathLibrary.MakeVector` _returnvalue_x_2 _returnvalue_y_2 (`KismetMathLibrary.Lerp` _returnvalue_z_2 (- (`self.actorZ`) (`self.hiddenAmount`)) _hidealpha))))
    (:`Finished`
      (`self.K2_DestroyActor`))))

(event `FlashOn`
  ;[1 1 1] If is hurt
  (if (`self.CanBehurt`)
    ;[1 1 1] switch to not hurt mat
    (`PrimitiveComponent.SetMaterial` (`self.Mesh`) 0 (`self.defaultMat`))
    (else
      ;[1 1 1] Change to hurt mat
      (`PrimitiveComponent.SetMaterial` (`self.Mesh`) 0 (`self.hurtMat`))
      (`KismetSystemLibrary.Delay` (`self.flashRate`))
      (`self.FlashOff`))))

(event `FlashOff`
  ;[1 1 1] If is hurt
  (if (`self.CanBehurt`)
    ;[1 1 1] Go to default mat
    (`PrimitiveComponent.SetMaterial` (`self.Mesh`) 0 (`self.defaultMat`))
    (else
      ;[1 1 1] Go to default mat then prepare to flash on
      (`PrimitiveComponent.SetMaterial` (`self.Mesh`) 0 (`self.defaultMat`))
      (`KismetSystemLibrary.Delay` (`self.flashRate`))
      (`self.FlashOn`))))

(event `self.ReceiveTick`
  (params (DeltaSeconds :type "Float (single-precision)"))
  (bind _returnvalue (`self.K2_GetActorRotation`))
  (bind (_returnvalue_roll _returnvalue_pitch _returnvalue_yaw) (`KismetMathLibrary.BreakRotator` (`KismetMathLibrary.RInterpTo` _returnvalue (`KismetMathLibrary.FindLookAtRotation` (`self.K2_GetActorLocation`) (`self.K2_GetActorLocation` (`self.currentTarget`))) DeltaSeconds 20.0)))
  (if (not (`self.isDead`))
    (`self.SwitchStates`
      (:`Attack`
        (if (not (`self.IsAttacking`))
          (`/Engine/EditorBlueprintResources/StandardMacros.IsValid` (`self.currentTarget`)
            (:`Is Valid`
              (`self.K2_SetActorRotation` (`KismetMathLibrary.MakeRotator` (.roll _returnvalue) (.pitch _returnvalue) _returnvalue_yaw)))))))))

(event `/Game/Student/Blueprint/Gameplay/Characters/Interfaces/BPI_Zombie.OnAnimAttackBegin`
  ;[1 1 1] on Attack animation begin and end
  (set `self.IsAttacking` true))

(event `/Game/Student/Blueprint/Gameplay/Characters/Interfaces/BPI_Zombie.OnAnimAttackEnd`
  ;[1 1 1] on Attack animation begin and end
  (set `self.IsAttacking` false))

(event `/Game/Student/Blueprint/Gameplay/Characters/Interfaces/BPI_Zombie.OnAttackContactEnd`
  ;[1 1 1] Animation attack events
  (`PrimitiveComponent.SetCollisionEnabled` (`self.attackCollison`) "NoCollision"))

(event `/Game/Student/Blueprint/Gameplay/Characters/Interfaces/BPI_Zombie.OnAttackContact`
  ;[1 1 1] Animation attack events
  (`PrimitiveComponent.SetCollisionEnabled` (`self.attackCollison`) "QueryAndPhysics")
  ;;[1 1 1] Incase the player hasn't moved to ensure overlap happens
  (`self.ApplyDamageInZone`))

(event `self.attackCollison.OnComponentBeginOverlap`
  (params (OverlappedComponent :type "PrimitiveComponent Object Reference") (OtherActor :type "Actor Object Reference") (OtherComp :type "PrimitiveComponent Object Reference") (OtherBodyIndex :type Integer) (bFromSweep :type Boolean) (SweepResult :type "HitResult Structure (by ref)"))
  ;[1 1 1] On attack collision overlap
  (bind _isonteam (message `/Game/Student/Blueprint/Interfaces/BPI_TeamData.IsOnTeam` OtherActor (`self.Team`)))
  (if (not _isonteam)
    (message `/Game/Student/Blueprint/Gameplay/Characters/Interfaces/BPI_Hurtable.DamageActor` OtherActor null 20.0 0.0 (0.0 0.0 0.0))))

(event `self.CapsuleComponent.OnComponentHit`
  (params (HitComponent :type "PrimitiveComponent Object Reference") (OtherActor :type "Actor Object Reference") (OtherComp :type "PrimitiveComponent Object Reference") (NormalImpulse :type "Vector Structure") (Hit :type "HitResult Structure (by ref)"))
  ;[1 1 1] On collsion capsule hit
  (`/Engine/EditorBlueprintResources/StandardMacros.IsValid` OtherActor
    (:`Is Valid`
      (bind _isonteam (message `/Game/Student/Blueprint/Interfaces/BPI_TeamData.IsOnTeam` OtherActor (`self.Team`)))
      (if _isonteam
        _
        (elif (`self.ActorHasTag` OtherActor "Player")
          (`self.SwitchStates`
            (:`Idle`
              _)
            (:`Chase`
              _))
          (set `self.currentTarget` OtherActor))))))

(event `/Game/Student/Blueprint/Gameplay/Characters/Interfaces/BPI_Hurtable.DamageActorDied`
  (params (DeadActor :type "Actor Object Reference"))
  ;[1 1 1] On target die
  (if (== DeadActor (`self.currentTarget`))
    (`self.GetNearestPlayer`)))

(fn `ApplyDamageInZone`
  (locals (Collisions :type "Array of EObjectTypeQuery Enum"))
  (bind (_aidata_attackrange _aidata_attackspeed _aidata_movememtspeed _aidata_mindamage _aidata_maxdamage) (break `/Game/Student/Blueprint/Gameplay/ZombieSurvival/AI/Data/S_ZombieData` (`self.AIData`)))
  (bind _outhits (`KismetSystemLibrary.SphereTraceMultiForObjects` (`SceneComponent.K2_GetComponentLocation` (`self.attackCollison`)) (* (`self.GetActorForwardVector`) (`SphereComponent.SphereRadius` (`self.attackCollison`))) (`SphereComponent.SphereRadius` (`self.attackCollison`)) (`local.Collisions`)))
  (for _array_element _outhits
    (bind _isonteam (message `/Game/Student/Blueprint/Interfaces/BPI_TeamData.IsOnTeam` (`.HitActor` (`GameplayStatics.BreakHitResult` _array_element)) (`self.Team`)))
    (if (not _isonteam)
      (message `/Game/Student/Blueprint/Gameplay/Characters/Interfaces/BPI_Hurtable.DamageActor` (`.HitActor` (`GameplayStatics.BreakHitResult` _array_element)) null (`KismetMathLibrary.RandomFloatInRange` _aidata_mindamage _aidata_maxdamage) 0.0 (0.0 0.0 0.0)))))

(fn `DoAttackAnim`
  (set `CharacterMovementComponent.MaxWalkSpeed` 0.0 (`self.CharacterMovement`))
  (`self.PlayAnimMontage` "/Game/Student/Assets/Animation/Zombie/M_ZombieAttack.M_ZombieAttack"))

(fn `EvaluateNewState`
  (`self.SwitchStates`
    (:`Idle`
      (`self.InitIdle`)
      (`PrimitiveComponent.SetCollisionEnabled` (`self.attackCollison`) "NoCollision"))
    (:`Chase`
      (`self.InitChase`)
      (`PrimitiveComponent.SetCollisionEnabled` (`self.attackCollison`) "NoCollision"))
    (:`Attack`
      (`self.InitAttack`))))

(fn `Get Alive Players`
  (returns (PlayersAlive :type "Array of /Game/Student/Blueprint/Gameplay/Characters/BP_BaseTeamCharacter Object Reference"))
  (locals (alivePlayers :type "Array of /Game/Student/Blueprint/Gameplay/Characters/BP_BaseTeamCharacter Object Reference"))
  (bind _players (message `/Game/Student/Blueprint/Interfaces/BPI_GameModeData.GetPlayers` (`GameplayStatics.GetGameMode`)))
  (for _array_element _players
    (bind _isalive (`/Game/Student/Blueprint/Gameplay/Characters/BP_BaseTeamCharacter.GetIsAlive` _array_element))
    (if _isalive
      (`KismetArrayLibrary.Array_Add` (`local.alivePlayers`) _array_element)))
  (return (`local.alivePlayers`)))

(fn `GetAction`
  (returns (state :type "/Game/Student/Blueprint/Gameplay/ZombieSurvival/AI/Data/E_ZombieStates Enum"))
  (return (`self.currentState`)))

(fn `GetCharMovement`
  (returns (movement :type "CharacterMovementComponent Object Reference"))
  (return (`self.CharacterMovement`)))

(fn `GetIsAlive`
  (returns (Alive :type Boolean))
  (if (`self.isDead`)
    (return false)
    (else
      (return true))))

(fn `GetNearestPlayer`
  (locals (CurrShortestDistance :type "Float (double-precision)") (playerAlive :type "Array of /Game/Student/Blueprint/Gameplay/Characters/BP_BaseTeamCharacter Object Reference") (shortestIndex :type Integer))
  (bind _output (`|GetArrayItem` (`local.playerAlive`) (`local.shortestIndex`)))
  (bind _playersalive (`self.Get Alive Players`))
  ;[1 1 1] Assume first element is the shortest distance
  (bind _output_get (set `local.playerAlive` _playersalive))
  (set `local.CurrShortestDistance` (`KismetMathLibrary.Vector_Distance` (`self.K2_GetActorLocation` (`|GetArrayItem` _output_get)) (`self.K2_GetActorLocation`)))
  (for (_array_element _array_index) (`local.playerAlive`)
    (bind _returnvalue (`KismetMathLibrary.Vector_Distance` (`self.K2_GetActorLocation` _array_element) (`self.K2_GetActorLocation`)))
    (if (<= _returnvalue (`local.CurrShortestDistance`))
      ;[1 1 1] Set the newest shortest distance and store index to element
      (set `local.CurrShortestDistance` _returnvalue)
      (set `local.shortestIndex` _array_index)))
  ;[1 1 1] Check if value is valid
  (`/Engine/EditorBlueprintResources/StandardMacros.IsValid` _output
    (:`Is Valid`
      ;[1 1 1] If it is chase target
      (set `self.currentTarget` _output)
      (`self.SetNewState` "NewEnumerator1"))
    (:`Is Not Valid`
      ;[1 1 1] Else be idle
      (`self.SetNewState` "NewEnumerator0"))))

(fn `GetScore`
  (returns (playerScore :type Integer))
  (return 0))

(fn `GetTeam`
  (returns (Team :type "/Game/Student/Blueprint/Data/E_Teams Enum"))
  (return "NewEnumerator0"))

(fn `GetZombieAIData`
  (returns (GetZombieData :type "/Game/Student/Blueprint/Gameplay/ZombieSurvival/AI/Data/S_ZombieData Structure") (GetCurrentTarget :type "Actor Object Reference"))
  (return (`self.AIData`) (`self.currentTarget`)))

(fn `InitAttack`
  (bind (_aidata_attackrange _aidata_attackspeed) (break `/Game/Student/Blueprint/Gameplay/ZombieSurvival/AI/Data/S_ZombieData` (`self.AIData`)))
  (if (`self.CanAttack`)
    (`self.DoAttackAnim`)
    (set `self.CanAttack` false)
    (elif (not (`KismetSystemLibrary.K2_IsTimerActiveHandle` (`self.MeleeAttackTimer`)))
      (bind _returnvalue (`KismetSystemLibrary.K2_SetTimer` null "ResetAttackMeleeCooldown" _aidata_attackspeed))
      (set `self.MeleeAttackTimer` _returnvalue)
      (set `CharacterMovementComponent.MaxWalkSpeed` 0.0 (`self.CharacterMovement`)))))

(fn `InitChase`
  (bind (_aidata_attackrange _aidata_attackspeed _aidata_movememtspeed) (break `/Game/Student/Blueprint/Gameplay/ZombieSurvival/AI/Data/S_ZombieData` (`self.AIData`)))
  (bind _isattacking (`self.IsAttacking`))
  (if (not _isattacking)
    (set `CharacterMovementComponent.MaxWalkSpeed` _aidata_movememtspeed (`self.CharacterMovement`))
    (set `self.IsAttacking` _isattacking)
    (set `self.CanAttack` true)))

(fn `InitIdle`
  (`MovementComponent.StopMovementImmediately` (`self.CharacterMovement`)))

(fn `IsOnTeam`
  (params (CallerTeam :type "/Game/Student/Blueprint/Data/E_Teams Enum" :default "NewEnumerator0"))
  (returns (IsOnTeam :type Boolean))
  ;[1 1 1] Evaluate whether te caller is on this team
  (return (== CallerTeam (`self.Team`))))

(fn `ResetAttackMeleeCooldown`
  (if (not (`self.CanAttack`))
    (set `self.CanAttack` true)))

(fn `ResetHurt`
  (set `self.CanBehurt` true))

(fn `SetNewState`
  (params (NewState :type "/Game/Student/Blueprint/Gameplay/ZombieSurvival/AI/Data/E_ZombieStates Enum" :default "NewEnumerator0"))
  (bind _output_get (set `self.currentState` NewState))
  (`self.OnStateChange` _output_get)
  (`self.EvaluateNewState`))

(fn `SetUp`
  (bind (_aidata_attackrange _aidata_attackspeed _aidata_movememtspeed _aidata_mindamage _aidata_maxdamage _aidata_maxhealth) (break `/Game/Student/Blueprint/Gameplay/ZombieSurvival/AI/Data/S_ZombieData` (`self.AIData`)))
  (set `CharacterMovementComponent.MaxWalkSpeed` _aidata_movememtspeed (`self.CharacterMovement`))
  (set `self.currentHealth` _aidata_maxhealth))

(fn `StartHurtTime`
  (bind _returnvalue (`KismetSystemLibrary.K2_SetTimer` null "ResetHurt" (`self.HurtTime`)))
  (set `self.HurtTimerHandle` _returnvalue))

(fn `TakeScore`
  (params (DecreaseAmount :type Integer))
  (returns (Valid :type Boolean))
  (return false))

(fn `UserConstructionScript`
  (set `self.defaultMat` (`|GetArrayItem` (`MeshComponent.GetMaterials` (`self.Mesh`)))))