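; Shop pickup that a player buys with score through an interaction.
; While the pickup is ready, overlapping its InteractSphere registers it as an interactable with Player-tagged actors and shows the shop name and cost; leaving clears both.
; Interact charges the cost through TakeScoreMessage, then refreshes the shop display and calls Pickup, starting the respawn timer if that succeeds.
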(event `self.InteractSphere.OnComponentBeginOverlap`
  (params (OverlappedComponent :type "PrimitiveComponent Object Reference") (OtherActor :type "Actor Object Reference") (OtherComp :type "PrimitiveComponent Object Reference") (OtherBodyIndex :type Integer) (bFromSweep :type Boolean) (SweepResult :type "HitResult Structure (by ref)"))
  (if (`self.pickupReady`)
    (`/Engine/EditorBlueprintResources/StandardMacros.IsValid` OtherActor
      (:`Is Valid`
        (if (`self.ActorHasTag` OtherActor "Player")
          (message `/Game/Student/Blueprint/Interfaces/BPI_Interact.NewInteractable` OtherActor self)
          (message `/Game/Student/Blueprint/Widgets/Interfaces/BPI_PlayerWidget.DisplayShop` OtherActor (`self.ShopName`) (`self.shopCost`)))))))

(event `self.InteractSphere.OnComponentEndOverlap`
  (params (OverlappedComponent :type "PrimitiveComponent Object Reference") (OtherActor :type "Actor Object Reference") (OtherComp :type "PrimitiveComponent Object Reference") (OtherBodyIndex :type Integer))
  (message `/Game/Student/Blueprint/Interfaces/BPI_Interact.NotInteractable` OtherActor self)
  (message `/Game/Student/Blueprint/Widgets/Interfaces/BPI_PlayerWidget.HideShop` OtherActor))

(event `/Game/Student/Blueprint/Interfaces/BPI_Interact.Interact`
  (params (NewInteractingPlayer :type "Actor Object Reference"))
  (bind _valid (message `/Game/Student/Blueprint/Gameplay/Characters/Interfaces/BPI_Scoreable.TakeScore` NewInteractingPlayer (`self.shopCost`)))
  (if _valid
    (message `/Game/Student/Blueprint/Widgets/Interfaces/BPI_PlayerWidget.DisplayShop` NewInteractingPlayer (`self.ShopName`) (`self.shopCost`))
    (bind _success (`self.Pickup` NewInteractingPlayer))
    (if _success
      (`self.SetRespawnTimer`))))

(fn `UserConstructionScript`
  (`parent.UserConstructionScript`))