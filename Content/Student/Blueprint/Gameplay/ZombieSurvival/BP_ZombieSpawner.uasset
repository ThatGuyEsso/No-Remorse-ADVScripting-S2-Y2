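; Zombie survival spawn point that players can temporarily seal with purchasable blockades.
; During waves, a randomized timer spawns AI-possessed zombies, gated by GameMode enemy-capacity events.
; Interacting costs score, then blockades drop in through a timeline one after another while the player stays in range, each paying a reward.
; A full set blocks spawning until, after a delay, blockades clear at random intervals, with spawning blocked until all are gone.
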(event `/Game/Student/Blueprint/Interfaces/BPI_Init.InitActor`
  ;[1 1 1] Init spawning
  (`self.SetUpBlockades`)
  (bind _zombiegamemode (message `/Game/Student/Blueprint/Interfaces/BPI_ZombieSurvival.GetZombieGameModeRef` (`GameplayStatics.GetGameMode`)))
  (add `/Game/Student/Blueprint/GameModes/GM_ZombieSurvial.OnEnemyCapacityReached` _zombiegamemode (delegate `OnCapacityReached`))
  (add `/Game/Student/Blueprint/GameModes/GM_ZombieSurvial.OnNotAtEnemyCapacity` _zombiegamemode (delegate `OnAvailableCapacity`))
  (add `/Game/Student/Blueprint/Spawning/BP_WaveManager.OnWaveStart` (`self.WaveManager`) (delegate `OnResetSpawnTimer`)))

(event `OnAvailableCapacity`
  ;[1 1 1] Init spawning
  ;;[0.09339 1 0.2877] On no longer at capacity
  (switch `/Game/Student/Blueprint/Spawning/E_WaveState` (`/Game/Student/Blueprint/Spawning/BP_WaveManager.WaveState` (`self.WaveManager`))
    (:`NewEnumerator0`
      (set `self.CanSpawn` true)
      (`self.OnResetSpawnTimer`))))

(event `OnCapacityReached`
  ;[1 1 1] Init spawning
  ;;[1 0.3407 0.4466] On Capacity Reached
  (set `self.CanSpawn` false))

(event `OnResetSpawnTimer`
  ;[1 1 1] On Reset timer
  (switch `/Game/Student/Blueprint/Spawning/E_WaveState` (`/Game/Student/Blueprint/Spawning/BP_WaveManager.WaveState` (`self.WaveManager`))
    (:`NewEnumerator0`
      (bind _returnvalue (`KismetSystemLibrary.K2_SetTimerDelegate` (delegate `OnSpawnZombie`) (`KismetMathLibrary.RandomFloatInRange` (`self.minSpawnTime`) (`self.maxSpawn`))))
      (set `self.SpawnTimer` _returnvalue))))

(event `OnSpawnZombie`
  ;[1 1 1] On Spawn Zombie
  (if (`self.CanSpawn`)
    (`self.SpawnZombie`)
    (`self.OnResetSpawnTimer`)))

(event `Build Baricade`
  (bind _output (`|GetArrayItem` (`self.Blockades`) (- (`self.nActiveBlockades`) 1)))
  (bind (_returnvalue_x _returnvalue_y _returnvalue_z) (`KismetMathLibrary.BreakVector` (`SceneComponent.K2_GetComponentLocation` _output)))
  (bind (_returnvalue_x_2 _returnvalue_y_2 _returnvalue_z_2) (`KismetMathLibrary.BreakVector` (`SceneComponent.K2_GetComponentLocation` _output)))
  ;[1 1 1] Get index of barricade
  (`self.EnableBarricade` _output)
  ;[1 1 1] Get original position
  (bind _output_get (set `self.originalBarricadeHeight` _returnvalue_z_2))
  (`SceneComponent.K2_SetWorldLocation` _output (`KismetMathLibrary.MakeVector` _returnvalue_x_2 _returnvalue_y_2 (+ _output_get (`self.buildHeight`))) false false)
  (bind (_direction _buildcurve) (`Timeline|BuildtimeLine` :!via `PlayFromStart`)
    (:`Update`
      ;[1 1 1] Lerp blockade down
      (`SceneComponent.K2_SetWorldLocation` _output (`KismetMathLibrary.MakeVector` _returnvalue_x _returnvalue_y (`KismetMathLibrary.Lerp` _returnvalue_z (`self.originalBarricadeHeight`) _buildcurve)) false false))
    (:`Finished`
      ;[1 1 1] Add score and check if player is still building
      (message `/Game/Student/Blueprint/Gameplay/Characters/Interfaces/BPI_Scoreable.AddScore` (`self.InteractingPlayer`) (`self.Reward`) null)
      (set `self.canBuild` true)
      (if (`self.isBuilding`)
        (`self.AddBlockade`)
        (if (>= (`self.nActiveBlockades`) (`KismetArrayLibrary.Array_Length` (`self.Blockades`)))
          (`KismetSystemLibrary.Delay` (`self.MaxRemoveTime`))
          (`self.BeginReducing Blockades`))))))

(event `self.InteractSphere.OnComponentBeginOverlap`
  (params (OverlappedComponent :type "PrimitiveComponent Object Reference") (OtherActor :type "Actor Object Reference") (OtherComp :type "PrimitiveComponent Object Reference") (OtherBodyIndex :type Integer) (bFromSweep :type Boolean) (SweepResult :type "HitResult Structure (by ref)"))
  ;[1 1 1] Check if not currently building and there is a valid player
  (if (not (`self.isBuilding`))
    (`/Engine/EditorBlueprintResources/StandardMacros.IsValid` OtherActor
      (:`Is Valid`
        (if (`self.ActorHasTag` OtherActor "Player")
          (`KismetArrayLibrary.Array_Add` (`self.PlayersInRange`) OtherActor)
          ;[1 1 1] Become interactable
          (message `/Game/Student/Blueprint/Interfaces/BPI_Interact.NewInteractable` OtherActor self)
          (set `self.canBuild` true)
          (message `/Game/Student/Blueprint/Widgets/Interfaces/BPI_PlayerWidget.DisplayShop` OtherActor (`self.Name`) (`self.buildCost`)))))))

(event `self.InteractSphere.OnComponentEndOverlap`
  (params (OverlappedComponent :type "PrimitiveComponent Object Reference") (OtherActor :type "Actor Object Reference") (OtherComp :type "PrimitiveComponent Object Reference") (OtherBodyIndex :type Integer))
  (bind _interactingplayer (`self.InteractingPlayer`))
  ;[1 1 1] Check if player leaving is building
  (`/Engine/EditorBlueprintResources/StandardMacros.IsValid` OtherActor
    (:`Is Valid`
      (`/Engine/EditorBlueprintResources/StandardMacros.IsValid` _interactingplayer
        (:`Is Valid`
          (if (== OtherActor _interactingplayer)
            ;[1 1 1] Update list of players and evaluate if the can still build
            (set `self.isBuilding` false)
            (`KismetArrayLibrary.Array_RemoveItem` (`self.PlayersInRange`) (`self.InteractingPlayer`))
            (message `/Game/Student/Blueprint/Interfaces/BPI_Interact.NotInteractable` (`self.InteractingPlayer`) self)
            (set `self.InteractingPlayer` null)
            (message `/Game/Student/Blueprint/Widgets/Interfaces/BPI_PlayerWidget.HideShop` OtherActor :!label _label)
            (if (<= (`KismetArrayLibrary.Array_Length` (`self.PlayersInRange`)) 0)
              (set `self.canBuild` false))
            (else
              (if (`self.ActorHasTag` OtherActor "Player") :!label _label_2
                (message `/Game/Student/Blueprint/Interfaces/BPI_Interact.NotInteractable` OtherActor self)
                (`KismetArrayLibrary.Array_RemoveItem` (`self.PlayersInRange`) OtherActor)
                (goto _label)))))
        (:`Is Not Valid`
          (goto _label_2))))))

(event `/Game/Student/Blueprint/Interfaces/BPI_Interact.Interact`
  (params (NewInteractingPlayer :type "Actor Object Reference"))
  ;[1 1 1] Validate if player is valid and if they have enough money
  (`/Engine/EditorBlueprintResources/StandardMacros.IsValid` (`self.InteractingPlayer`)
    (:`Is Not Valid`
      (bind _playerscore (message `/Game/Student/Blueprint/Gameplay/Characters/Interfaces/BPI_Scoreable.GetScore` NewInteractingPlayer))
      ;[1 1 1] If they can rededuce score and add blockade
      (if (>= _playerscore (`self.buildCost`))
        (bind _output_get (set `self.InteractingPlayer` NewInteractingPlayer))
        (message `/Game/Student/Blueprint/Gameplay/Characters/Interfaces/BPI_Scoreable.TakeScore` _output_get (`self.buildCost`))
        (`self.AddBlockade`)
        (message `/Game/Student/Blueprint/Widgets/Interfaces/BPI_PlayerWidget.DisplayShop` NewInteractingPlayer (`self.Name`) (`self.buildCost`))))))

(event `BeginReducing Blockades`
  (if (`self.isBuilding`)
    (set `self.isClearing` false)
    (else
      (set `self.isClearing` true)
      (`self.RemoveBlockade`)
      (if (<= (`self.nActiveBlockades`) 0)
        (set `self.isClearing` false)
        (else
          (`KismetSystemLibrary.Delay` (`KismetMathLibrary.RandomFloatInRange` (`self.minRemoveTime`) (`self.MaxRemoveTime`)))
          (`self.BeginReducing Blockades`))))))

(fn `AddBlockade`
  (if (and (< (`self.nActiveBlockades`) (`KismetArrayLibrary.Array_Length` (`self.Blockades`))) (== (`self.canBuild`) true))
    (`/Engine/EditorBlueprintResources/StandardMacros.IncrementInt` (`self.nActiveBlockades`)
      (:`  `
        (set `self.isBuilding` true)
        (set `self.canBuild` false)
        (`self.Build Baricade`)))
    (else
      (set `self.isBuilding` false))))

(fn `EnableBarricade`
  (params (barricade :type "StaticMeshComponent Object Reference"))
  (`/Engine/EditorBlueprintResources/StandardMacros.IsValid` barricade
    (:`Is Valid`
      (`SceneComponent.SetVisibility` barricade true false)
      (`PrimitiveComponent.SetCollisionEnabled` barricade "QueryAndPhysics"))))

(fn `GetPlayers`
  (returns (Players :type "Array of /Game/Student/Blueprint/Gameplay/Characters/BP_BaseTeamCharacter Object Reference"))
  (return))

(fn `GetScore`
  (returns (playerScore :type Integer))
  (return 0))

(fn `GetZombieAIData`
  (returns (GetZombieData :type "/Game/Student/Blueprint/Gameplay/ZombieSurvival/AI/Data/S_ZombieData Structure") (GetCurrentTarget :type "Actor Object Reference"))
  (return (struct) null))

(fn `GetZombieGameModeRef`
  (returns (ZombieGameMode :type "/Game/Student/Blueprint/GameModes/GM_ZombieSurvial Object Reference"))
  (return null))

(fn `IsAtZombieCapacity`
  (returns (IsAtCapacity :type Boolean))
  (return false))

(fn `IsBlocked`
  (returns (isblocked :type Boolean))
  (if (or (>= (`self.nActiveBlockades`) (`KismetArrayLibrary.Array_Length` (`self.Blockades`))) (`self.isClearing`))
    (return true)
    (else
      (return false))))

(fn `RemoveBlockade`
  (bind _output (`|GetArrayItem` (`self.Blockades`) (`KismetMathLibrary.Clamp` (- (`self.nActiveBlockades`) 1) 0 (`KismetArrayLibrary.Array_Length` (`self.Blockades`)))))
  (`/Engine/EditorBlueprintResources/StandardMacros.IsValid` _output
    (:`Is Valid`
      (`SceneComponent.SetVisibility` _output false false)
      (`PrimitiveComponent.SetCollisionEnabled` _output "NoCollision")
      (bind _result (`/Engine/EditorBlueprintResources/StandardMacros.DecrementInt` (`self.nActiveBlockades`))
        (:`  `
          (set `self.nActiveBlockades` (`KismetMathLibrary.Clamp` _result 0 (`KismetArrayLibrary.Array_Length` (`self.Blockades`)))))))))

(fn `SetSpawnRateBounds`
  (params (minSpawnTime :type "Float (double-precision)") (maxSpawn :type "Float (double-precision)"))
  (set `self.minSpawnTime` minSpawnTime)
  (set `self.maxSpawn` maxSpawn))

(fn `SetUpBlockades`
  (bind _blockades (`self.Blockades`))
  (`KismetArrayLibrary.Array_Clear` (`self.Blockades`))
  (`|ExecutionSequence`
    (:`then_0`
      (`KismetArrayLibrary.Array_Add` _blockades (`self.Blockade`))
      (`KismetArrayLibrary.Array_Add` _blockades (`self.Blockade1`))
      (`KismetArrayLibrary.Array_Add` _blockades (`self.Blockade2`))
      (set `self.nActiveBlockades` (`KismetArrayLibrary.Array_Length` (`self.Blockades`)))
      (for _ (`self.Blockades`)
        (`self.RemoveBlockade`)))))

(fn `SpawnZombie`
  (locals (currentController :type "/Game/Student/Blueprint/Controllers/AIC_ZombieController Object Reference") (CurrentZombie :type "/Game/Student/Blueprint/Gameplay/Characters/BP_Zombie Object Reference"))
  (bind _currentzombie (`local.CurrentZombie`))
  (bind _isblocked (`self.IsBlocked`))
  (if _isblocked
    (`KismetSystemLibrary.PrintString` "Blocked or clearing" true true (struct :`R` 1.0 :`B` 0.024402 :`A` 1.0))
    (else
      (bind _returnvalue (`|SpawnActorFromClass` "/Game/Student/Blueprint/Controllers/AIC_ZombieController.AIC_ZombieController_C" (`KismetMathLibrary.MakeTransform` (0.0 0.0 0.0)) "Undefined" "OverrideRootScale" null null))
      (set `local.currentController` _returnvalue)
      (bind _returnvalue_2 (`|SpawnActorFromClass` "/Game/Student/Blueprint/Gameplay/Characters/BP_Zombie.BP_Zombie_C" (`KismetMathLibrary.MakeTransform` (`SceneComponent.K2_GetComponentLocation` (`self.SpawnPoint`))) "Undefined" "OverrideRootScale" null null))
      (bind _output_get (set `local.CurrentZombie` _returnvalue_2))
      (`Controller.Possess` (`local.currentController`) _output_get)
      (`/Game/Student/Blueprint/Gameplay/Characters/BP_Zombie.SetUp` (`local.CurrentZombie`))
      (`/Game/Student/Blueprint/Controllers/AIC_ZombieController.InitController` (`local.currentController`))
      (message `/Game/Student/Blueprint/Interfaces/BPI_ZombieSurvival.NewZombieSpawned` (`GameplayStatics.GetGameMode`))
      (message `/Game/Student/Blueprint/Interfaces/BPI_TeamData.AssignTeam` _currentzombie "NewEnumerator3")
      (`/Game/Student/Blueprint/Gameplay/Characters/BP_Zombie.GetNearestPlayer` _currentzombie))))

(fn `TakeScore`
  (params (DecreaseAmount :type Integer))
  (returns (Valid :type Boolean))
  (return false))

(fn `UserConstructionScript`)