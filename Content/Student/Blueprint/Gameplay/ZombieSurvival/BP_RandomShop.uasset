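; BP_RandomShop is a zombie survival shop that gives a random pickup to the actor passed to its Pickup function.
; Pickup sets the PickupActor child actor to a random class from PossiblePickUps, then calls Pickup on the spawned BasePickup and returns its result, or false if no child actor is valid.
; The Interact event only defers to the parent class.
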(event `/Game/Student/Blueprint/Interfaces/BPI_Interact.Interact`
  (params (NewInteractingPlayer :type "Actor Object Reference"))
  (`parent.Interact` NewInteractingPlayer))

(fn `Pickup`
  (params (Actor :type "Actor Object Reference"))
  (returns (Success :type Boolean))
  (bind _childactor (`ChildActorComponent.ChildActor` (`self.PickupActor`)))
  (`ChildActorComponent.SetChildActorClass` (`self.PickupActor`) (`|GetArrayItem` (`self.PossiblePickUps`) (`KismetMathLibrary.RandomIntegerInRange` 0 (`KismetArrayLibrary.Array_LastIndex` (`self.PossiblePickUps`)))))
  (`/Engine/EditorBlueprintResources/StandardMacros.IsValid` _childactor
    (:`Is Valid`
      (bind _success (`/Game/Framework_Blueprints/Pickups/BasePickup.Pickup` (cast `/Game/Framework_Blueprints/Pickups/BasePickup` _childactor :!pure true) Actor))
      (return _success))
    (:`Is Not Valid`
      (return false))))

(fn `UserConstructionScript`
  (`parent.UserConstructionScript`))