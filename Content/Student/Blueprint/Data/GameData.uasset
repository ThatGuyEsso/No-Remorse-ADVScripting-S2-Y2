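; GameData Blueprint holds session state for a two-player minigame series: setup data, each player's score and colour, and games left.
; Events update setup fields, player data and the remaining-games counter, while getters expose them.
; GenerateGameModeList builds the play order by rotating Zombie Survival, Boss Rush and King of the Hill from the chosen first mode.
; ResetData clears player data and the counter, leaving setup and sequence intact.
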(event `/Game/Student/Blueprint/Interfaces/BPI_GameData.SetSetUpData`
  (params (Data :type "/Game/Student/Blueprint/Data/S_SetUpData Structure"))
  (set `self.SetUpData` Data))

(event `/Game/Student/Blueprint/Interfaces/BPI_GameData.SetPlayerOne`
  (params (PlayerOne :type "/Game/Student/Blueprint/Data/S_ControllerMap Structure"))
  (`self.UpdatePlayerOne` PlayerOne))

(event `/Game/Student/Blueprint/Interfaces/BPI_GameData.SetNPlayers`
  (params (nPlayer :type Integer))
  (`self.UpdateNPlayers` nPlayer))

(event `/Game/Student/Blueprint/Interfaces/BPI_GameData.UpdatePlayerOneData`
  (params (PlayerOneData :type "/Game/Student/Blueprint/Data/S_PlayerData Structure"))
  (bind _playeronedata_playerscore (break `/Game/Student/Blueprint/Data/S_PlayerData` (`self.PlayerOneData`)))
  (set `self.PlayerOneData` (make `/Game/Student/Blueprint/Data/S_PlayerData` (+ _playeronedata_playerscore PlayerOneData_PlayerScore_6_7764934C4471CFF05C22148C967594F4) PlayerOneData_PlayerColour_5_F8D8D5A242847EF448AAE992D248BB5D)))

(event `/Game/Student/Blueprint/Interfaces/BPI_GameData.UpdatePlayerTwoData`
  (params (PlayerTwoData :type "/Game/Student/Blueprint/Data/S_PlayerData Structure"))
  (bind _playertwodata_playerscore (break `/Game/Student/Blueprint/Data/S_PlayerData` (`self.PlayerTwoData`)))
  (set `self.PlayerTwoData` (make `/Game/Student/Blueprint/Data/S_PlayerData` (+ PlayerTwoData_PlayerScore_6_7764934C4471CFF05C22148C967594F4 _playertwodata_playerscore) PlayerTwoData_PlayerColour_5_F8D8D5A242847EF448AAE992D248BB5D)))

(event `/Game/Student/Blueprint/Interfaces/BPI_GameData.SetTotalGames`
  (params (totalGames :type Integer))
  (set `self.GamesLeft` totalGames))

(event `/Game/Student/Blueprint/Interfaces/BPI_GameData.DecrementGamesLeft`
  (`/Engine/EditorBlueprintResources/StandardMacros.DecrementInt` (`self.GamesLeft`)))

(event `/Game/Student/Blueprint/Interfaces/BPI_GameData.ResetData`
  (set `self.GamesLeft` 0)
  (set `self.PlayerTwoData` (struct))
  (set `self.PlayerOneData` (struct)))

(event `/Game/Student/Blueprint/Interfaces/BPI_GameData.GenerateLevelSequence`
  (params (InitialLevelSequence :type "/Game/Student/Blueprint/Data/E_GameModes Enum" :default "NewEnumerator0"))
  (`self.GenerateGameModeList` InitialLevelSequence))

(fn `GenerateGameModeList`
  (params (initGame :type "/Game/Student/Blueprint/Data/E_GameModes Enum" :default "NewEnumerator0"))
  (`KismetArrayLibrary.Array_Clear` (`self.GameModeSequence`))
  (`KismetArrayLibrary.Array_Add` (`self.GameModeSequence`) initGame)
  (switch `/Game/Student/Blueprint/Data/E_GameModes` (`|GetArrayItem` (`self.GameModeSequence`))
    (:`NewEnumerator0`
      (`KismetArrayLibrary.Array_Add` (`self.GameModeSequence`) "NewEnumerator1")
      (`KismetArrayLibrary.Array_Add` (`self.GameModeSequence`) "NewEnumerator2"))
    (:`NewEnumerator1`
      (`KismetArrayLibrary.Array_Add` (`self.GameModeSequence`) "NewEnumerator2")
      (`KismetArrayLibrary.Array_Add` (`self.GameModeSequence`) "NewEnumerator0"))
    (:`NewEnumerator2`
      (`KismetArrayLibrary.Array_Add` (`self.GameModeSequence`) "NewEnumerator0")
      (`KismetArrayLibrary.Array_Add` (`self.GameModeSequence`) "NewEnumerator1"))))

(fn `GetGamesTotal`
  (returns (totalGames :type Integer))
  (return (`KismetArrayLibrary.Array_Length` (`self.GameModeSequence`))))

(fn `GetNextGameMode`
  (params (index :type Integer))
  (returns (GameMode :type "/Game/Student/Blueprint/Data/E_GameModes Enum"))
  (return (`|GetArrayItem` (`self.GameModeSequence`) index)))

(fn `GetNumberOfGamesLeft`
  (returns (GamesLeft :type Integer))
  (return (`self.GamesLeft`)))

(fn `GetPlayerData`
  (returns (PlayerOne :type "/Game/Student/Blueprint/Data/S_PlayerData Structure") (PlayerTwo :type "/Game/Student/Blueprint/Data/S_PlayerData Structure"))
  (return (`self.PlayerOneData`) (`self.PlayerTwoData`)))

(fn `GetSetUpData`
  (returns (Data :type "/Game/Student/Blueprint/Data/S_SetUpData Structure"))
  (return (`self.SetUpData`)))

(fn `UpdateNPlayers`
  (params (`Set Up Data N Players` :type Integer))
  (locals (currentPlayerOne :type "/Game/Student/Blueprint/Data/S_ControllerMap Structure"))
  (bind (_setupdata_nplayers _setupdata_playerone) (break `/Game/Student/Blueprint/Data/S_SetUpData` (`self.SetUpData`)))
  (bind _output_get (set `local.currentPlayerOne` _setupdata_playerone))
  (set `self.SetUpData` (make `/Game/Student/Blueprint/Data/S_SetUpData` `Set Up Data N Players` _output_get)))

(fn `UpdatePlayerOne`
  (params (`Set Up Data Player One` :type "/Game/Student/Blueprint/Data/S_ControllerMap Structure"))
  (locals (currentPlayers :type Integer))
  (bind _setupdata_nplayers (break `/Game/Student/Blueprint/Data/S_SetUpData` (`self.SetUpData`)))
  (bind _output_get (set `local.currentPlayers` _setupdata_nplayers))
  (set `self.SetUpData` (make `/Game/Student/Blueprint/Data/S_SetUpData` _output_get `Set Up Data Player One`)))