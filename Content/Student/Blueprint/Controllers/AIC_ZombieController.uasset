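; AI controller for zombie pawns that runs the BT_Zombie behavior tree.
; InitController starts the tree and seeds the ZombieStates blackboard enum with the pawn's default AI state, read through the GetZombieAIData message.
; It then binds to BP_Zombie's state-change event so each new state is written to the same blackboard key.
; BeginDeath destroys the controller.
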(event `OnInit`
  (bind _asbp_zombie (cast `/Game/Student/Blueprint/Gameplay/Characters/BP_Zombie` (`self.K2_GetPawn`)))
  (add `/Game/Student/Blueprint/Gameplay/Characters/BP_Zombie.OnStateChange` _asbp_zombie (delegate `OnStateChange`)))

(event `OnStateChange`
  (params (State :type "/Game/Student/Blueprint/Gameplay/ZombieSurvival/AI/Data/E_ZombieStates Enum" :default "NewEnumerator0"))
  (`BlackboardComponent.SetValueAsEnum` (`AIBlueprintHelperLibrary.GetBlackboard` null) "ZombieStates" State))

(event `/Game/Student/Blueprint/Gameplay/Characters/Interfaces/BPI_Zombie.BeginDeath`
  (`self.K2_DestroyActor`))

(fn `GetZombieAIData`)

(fn `InitController`
  (`self.RunBehaviorTree` "/Game/Student/Blueprint/Gameplay/ZombieSurvival/AI/BT_Zombie.BT_Zombie")
  (bind _getzombiedata (message `/Game/Student/Blueprint/Gameplay/Characters/Interfaces/BPI_Zombie.GetZombieAIData` (`self.K2_GetPawn`)))
  (`BlackboardComponent.SetValueAsEnum` (`AIBlueprintHelperLibrary.GetBlackboard` null) "ZombieStates" (`.DefaultAIState_31_0528A6C645AEBAC6B5B9DAA0FAFE68D0` (break `/Game/Student/Blueprint/Gameplay/ZombieSurvival/AI/Data/S_ZombieData` _getzombiedata)))
  (`self.OnInit`))

(fn `UserConstructionScript`)