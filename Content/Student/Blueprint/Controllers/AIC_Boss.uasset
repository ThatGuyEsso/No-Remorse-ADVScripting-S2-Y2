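; AIC_Boss is the AI controller for the boss pawn and drives it with the BT_Boss behavior tree.
; Init starts the tree, seeds the BossStates blackboard key from the pawn's boss data, then runs OnInit.
; OnInit binds to BP_Boss state-change events so each new state is mirrored into that blackboard key.
; OnDestroy unpossesses the pawn and destroys the controller.
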(event `OnInit`
  (bind _asbp_boss (cast `/Game/Student/Blueprint/Gameplay/BossRush/Boss/BP_Boss` (`self.K2_GetPawn`)))
  (add `/Game/Student/Blueprint/Gameplay/BossRush/Boss/BP_Boss.OnStateChange` _asbp_boss (delegate `OnNewState`)))

(event `OnNewState`
  (params (State :type "/Game/Student/Blueprint/Gameplay/BossRush/Boss/E_BossState Enum" :default "NewEnumerator0"))
  (`BlackboardComponent.SetValueAsEnum` (`AIBlueprintHelperLibrary.GetBlackboard` null) "BossStates" State))

(event `OnDestroy`
  (`self.UnPossess`)
  (`self.K2_DestroyActor`))

(fn `Init`
  (`self.RunBehaviorTree` "/Game/Student/Blueprint/Gameplay/BossRush/Boss/BT_Boss.BT_Boss")
  (bind (_defaultstate _currentstate) (message `/Game/Student/Blueprint/Gameplay/BossRush/Boss/BPI_Boss.GetBossData` (`self.K2_GetPawn`)))
  (`BlackboardComponent.SetValueAsEnum` (`AIBlueprintHelperLibrary.GetBlackboard` null) "BossStates" _currentstate)
  (`self.OnInit`))

(fn `UserConstructionScript`)