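; Player controller that relays input actions as messages, covering controller registration, character actions and selection navigation.
; Jump and Dash go to the controlled pawn, while RegisterController, Select and the four directional inputs go to the game mode.
; SetID stores a controller ID and marks it registered; GetControlloerID returns that state, with an ID of zero when unregistered.
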(event `InputAction|RegisterController`
  (params (Key :type "Key Structure"))
  (:`Released`
    (message `/Game/Student/Blueprint/Interfaces/BPI_MainMenu.RegisterController` (`GameplayStatics.GetGameMode`) self)))

(event `InputAction|Jump`
  (params (Key :type "Key Structure"))
  (:`Pressed`
    (message `/Game/Student/Blueprint/Gameplay/Characters/Interfaces/BPI_CharacterActions.OnJump` (`self.K2_GetPawn`))))

(event `InputAction|Dash`
  (params (Key :type "Key Structure"))
  (:`Pressed`
    (message `/Game/Student/Blueprint/Gameplay/Characters/Interfaces/BPI_CharacterActions.OnDash` (`self.K2_GetPawn`))))

(event `InputAction|Select`
  (params (Key :type "Key Structure"))
  (:`Pressed`
    (message `/Game/Student/Blueprint/Interfaces/BPI_WidgetButtonControl.Select` (`GameplayStatics.GetGameMode`))))

(event `InputAction|NextButton`
  (params (Key :type "Key Structure"))
  (:`Pressed`
    (message `/Game/Student/Blueprint/Interfaces/BPI_WidgetButtonControl.MoveRight` (`GameplayStatics.GetGameMode`))))

(event `InputAction|PrevButton`
  (params (Key :type "Key Structure"))
  (:`Pressed`
    (message `/Game/Student/Blueprint/Interfaces/BPI_WidgetButtonControl.MoveLeft` (`GameplayStatics.GetGameMode`))))

(event `InputAction|BelowButton`
  (params (Key :type "Key Structure"))
  (:`Pressed`
    (message `/Game/Student/Blueprint/Interfaces/BPI_WidgetButtonControl.MoveDown` (`GameplayStatics.GetGameMode`))))

(event `InputAction|AboveButton`
  (params (Key :type "Key Structure"))
  (:`Pressed`
    (message `/Game/Student/Blueprint/Interfaces/BPI_WidgetButtonControl.MoveUp` (`GameplayStatics.GetGameMode`))))

(fn `GetControlloerID`
  (returns (isRegistered :type Boolean) (controllerID :type Integer))
  (if (`self.isRegistered`)
    (return (`self.isRegistered`) (`self.controllerID`))
    (else
      (return false 0))))

(fn `SetID`
  (params (controllerID :type Integer))
  (set `self.controllerID` controllerID)
  (set `self.isRegistered` true))

(fn `UserConstructionScript`)