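; Base character for a twin-stick shooter, handling movement, stick-aimed rotation, weapons, health and pickups.
; Weapon actors sit on hand and holster sockets, cycle through timed montage swaps, and refire held shots via cooldown events rather than Tick.
; Damage flashes a dynamic team-coloured material, updates the health widget, and triggers ragdoll and weapon drop before destruction.
; Init spawns default weapons and sets up health, but BeginPlay leaves it unconnected; F/G are debug heal/damage keys.
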(event `self.ReceiveBeginPlay`
  ;[1 1 1] Initilise Character
)

(event `InputAxis|MoveRight`
  (params (AxisValue :type "Float (single-precision)"))
  ;[1 1 1] Move and Rotate Input
  (`PawnMovementComponent.AddInputVector` (`self.CharacterMovement`) (`KismetMathLibrary.MakeVector` 0.0 AxisValue) false))

(event `InputAction|Fire`
  (params (Key :type "Key Structure"))
  ;[1 1 1] Action Inputs
  (:`Pressed`
    (set `self.fireHeld` true)
    (`self.TryFire`))
  (:`Released`
    (set `self.fireHeld` false)))

(event `InputAction|ChangeWeaponUp`
  (params (Key :type "Key Structure"))
  ;[1 1 1] Action Inputs
  (:`Pressed`
    (`self.ChangeWeapon` 1)))

(event `InputAxis|MoveForward`
  (params (AxisValue :type "Float (single-precision)"))
  ;[1 1 1] Move and Rotate Input
  (`PawnMovementComponent.AddInputVector` (`self.CharacterMovement`) (`KismetMathLibrary.MakeVector` AxisValue) false)
  (`self.InputRotation`))

(event `InputAction|ChangeWeaponDown`
  (params (Key :type "Key Structure"))
  ;[1 1 1] Action Inputs
  (:`Pressed`
    (`self.ChangeWeapon` -1)))

(event `PlayFireAnim`
  ;[1 1 1] Animation montages
  (`|PlayMontage` (`self.Mesh`) "/Game/ArtAssets/AlienCharacter/Animations/Montage_Fire.Montage_Fire"))

(event `self.ReceiveAnyDamage`
  (params (Damage :type "Float (single-precision)") (DamageType :type "DamageType Object Reference") (InstigatedBy :type "Controller Object Reference") (DamageCauser :type "Actor Object Reference"))
  ;[1 0.5289 0.499] Damage functionality
  (`self.FlashDamage`)
  (set `self.health` (- (`self.health`) Damage))
  (`/Game/Framework_Blueprints/UI/CharacterHealth.UpdateHealthbars` (`self.HealthUI`) (`self.health`) (`self.MaxHealth`)) ; Update Health Widget
  (if (<= (`self.health`) 0.0)
    (set `self.dead` true)
    ;[1 1 1] Handle Physics on Death
    (`self.HandlePhysicsOnDeath`)
    (`KismetSystemLibrary.Delay` 2.0)
    (for _array_element (`self.Weapons`)
      (`self.K2_DestroyActor` _array_element))
    (`self.K2_DestroyActor`)))

(event `PlayChangeWeapAnim`
  ;[1 1 1] Animation montages
  (`|PlayMontage` (`self.Mesh`) "/Game/ArtAssets/AlienCharacter/Animations/Montage_ChangeWeap.Montage_ChangeWeap"))

(event `FlashDamage`
  ;[1 1 1] When we take damage, flash character
  (bind (_direction _alpha) (`Timeline|AlphaFlash` :!via `PlayFromStart`)
    (:`Update`
      (`MaterialInstanceDynamic.SetScalarParameterValue` (`self.DynamicMaterial`) "FlashAlpha" _alpha))))

(event `Key|F`
  (params (Key :type "Key Structure"))
  ;[1 1 1] Debug inputs
  (:`Pressed`
    (`self.AddHealth` 25.0)))

(event `Key|G`
  (params (Key :type "Key Structure"))
  ;[1 1 1] Debug inputs
  (:`Pressed`
    (`GameplayStatics.ApplyDamage` self 8.0)))

(fn `AddHealth`
  (params (health :type "Float (double-precision)"))
  (set `self.health` (`KismetMathLibrary.FClamp` (+ (`self.health`) health) 0.0 (`self.MaxHealth`)))
  (`/Game/Framework_Blueprints/UI/CharacterHealth.UpdateHealthbars` (`self.HealthUI`) (`self.health`) (`self.MaxHealth`)))

(fn `AddNewWeapon`
  (params (inHand :type Boolean) (Class :type "/Game/Framework_Blueprints/Weapons/Weapon_Base Class Reference"))
  (bind _returnvalue (`|SpawnActorFromClass` Class (`KismetMathLibrary.MakeTransform` (0.0 0.0 0.0)) "AlwaysSpawn" "OverrideRootScale" null null))
  (`KismetArrayLibrary.Array_Add` (`self.Weapons`) _returnvalue)
  (`/Game/Framework_Blueprints/Weapons/Weapon_Base.Init` _returnvalue self)
  (if inHand
    (`self.K2_AttachToComponent` _returnvalue (`self.Mesh`) "RightHandSocket" "SnapToTarget" "SnapToTarget" "KeepWorld" true)
    (else
      (`self.K2_AttachToComponent` _returnvalue (`self.Mesh`) "HolsterSocket" "SnapToTarget" "SnapToTarget" "KeepWorld" true))))

(fn `ChangeWeapon`
  (params (next :type Integer))
  (returns (Changed :type Boolean))
  (bind _returnvalue (+ (`self.currentWeapon`) next))
  (if (and (not (`self.changingWeapons`)) (or (> (`KismetArrayLibrary.Array_Length` (`self.Weapons`)) 1) (== next 0)))
    (set `self.PreviousWeapon` (`self.currentWeapon`))
    (if (< _returnvalue 0)
      (set `self.currentWeapon` (`KismetArrayLibrary.Array_LastIndex` (`self.Weapons`))) ; loop back to last weapon in the array
      (elif (> _returnvalue (`KismetArrayLibrary.Array_LastIndex` (`self.Weapons`)))
        (set `self.currentWeapon` 0) ; loop back to first weapon in the array
        (else
          (set `self.currentWeapon` _returnvalue) ; Select next or previous
        )))
    (`self.PlayChangeWeapAnim`)
    (`self.OnChangedWeapon` (`|GetArrayItem` (`self.Weapons`) (`self.currentWeapon`)))
    (set `self.changingWeapons` true)
    (`KismetSystemLibrary.K2_SetTimerDelegate` (`|CreateDelegate` :!event `UpdateWeaponActors`) 0.3) ; Delay for weapon change animation
    (`KismetSystemLibrary.K2_SetTimerDelegate` (`|CreateDelegate` :!event `CompleteWeaponSwap`) 0.9) ; Delay for weapon change animation
    (return true)
    (else
      (return false))))

(fn `CompleteWeaponSwap`
  (set `self.changingWeapons` false)
  (`self.TryWeaponRefire`) ; continue firing if fire is held after swap
)

(fn `GetFirePoint`
  (returns (NewParam :type "Transform Structure"))
  (return (`SceneComponent.K2_GetComponentToWorld` (`self.FirePoint`))))

(fn `HandlePhysicsOnDeath`
  (bind _mesh (`self.Mesh`))
  (`PrimitiveComponent.SetSimulatePhysics` _mesh true)
  (`PrimitiveComponent.SetCollisionEnabled` _mesh "PhysicsOnly")
  (`PrimitiveComponent.SetCollisionEnabled` (`self.CapsuleComponent`) "NoCollision")
  (for _array_element (`self.Weapons`)
    (`/Game/Framework_Blueprints/Weapons/Weapon_Base.DropWeaponPhysics` _array_element)
    (`self.K2_DetachFromActor` _array_element "KeepRelative" "KeepRelative" "KeepRelative")))

(fn `Init`
  ;[1 1 1] Set default health
  (set `self.health` (`self.MaxHealth`))
  (`self.SetupMaterial`)
  ;[1 1 1] Add weapons to our character from default class
  ; Change the default weapon to change the wepaon we spawn with
  (for (_array_element _array_index) (`self.DefaultWeapons`)
    (`self.AddNewWeapon` (== _array_index 0) _array_element))
  ;[1 1 1] Change the wepaon
  (`self.ChangeWeapon` 0)
  ;[1 1 1] Update our spatial health widgets.
  (bind _output_get (set `self.HealthUI` (cast `/Game/Framework_Blueprints/UI/CharacterHealth` (`WidgetComponent.GetUserWidgetObject` (`self.HealthWidget`)) :!pure true)))
  (`PrimitiveComponent.SetCastShadow` (`self.HealthWidget`) false)
  (`/Game/Framework_Blueprints/UI/CharacterHealth.UpdateHealthbars` _output_get (`self.health`) (`self.MaxHealth`)))

(fn `InputRotation`
  (bind _returnvalue (`KismetMathLibrary.MakeVector` (`self.GetInputAxisValue`) (`self.GetInputAxisValue`)))
  (if (> (`KismetMathLibrary.VSize` _returnvalue) (`self.RotationDeadzone`))
    (`self.K2_SetActorRotation` (`KismetMathLibrary.RLerp` (`self.K2_GetActorRotation`) (`KismetMathLibrary.Conv_VectorToRotator` _returnvalue) (* (`GameplayStatics.GetWorldDeltaSeconds`) (`self.CharacterRotationSpeed`)) true)) ; This could instead use controller rotation, ie in pawn default properties tick 'UseControllerRotationYaw' and then get/set controllerRotation\nJust using all pawn stuff for the moment
  ))

(fn `PickUpAmmo`
  (params (PercentRefill :type "Float (double-precision)"))
  (returns (Success :type Boolean))
  (for _array_element (`self.Weapons`)
    (`/Game/Framework_Blueprints/Weapons/Weapon_Base.AddAmmoPercent` _array_element PercentRefill))
  (`self.OnWeaponFired` (`|GetArrayItem` (`self.Weapons`) (`self.currentWeapon`))) ; UI update ammo
  (return true))

(fn `PickUpHealth`
  (params (AmountH :type "Float (double-precision)"))
  (returns (Success :type Boolean))
  (if (< (`self.health`) (`self.MaxHealth`))
    (`self.AddHealth` AmountH)
    (return true)
    (else
      (return false))))

(fn `PickUpSpecificAmmo`
  (params (Weapon :type "/Game/Framework_Blueprints/Weapons/Weapon_Base Object Reference") (Percent :type "Float (double-precision)"))
  (returns (Success :type Boolean))
  (if (< (`/Game/Framework_Blueprints/Weapons/Weapon_Base.Ammo` Weapon) (`/Game/Framework_Blueprints/Weapons/Weapon_Base.MaxAmmo` Weapon))
    (`/Game/Framework_Blueprints/Weapons/Weapon_Base.AddAmmoPercent` Weapon Percent)
    (return true)
    (else
      (return false))))

(fn `PickUpWeapon`
  (params (Weapon :type "/Game/Framework_Blueprints/Weapons/Weapon_Base Object Reference"))
  (returns (Success :type Boolean))
  (bind _returnvalue (`GameplayStatics.GetObjectClass` Weapon))
  (for _array_element (`self.Weapons`)
    (if (== _returnvalue (`GameplayStatics.GetObjectClass` _array_element))
      (bind _success (`self.PickUpSpecificAmmo` _array_element 0.5)) ; has the weapon already, add ammo
      (if _success
        (if (== (`|GetArrayItem` (`self.Weapons`) (`self.currentWeapon`)) _array_element)
          (`self.OnWeaponFired` _array_element) ; to update ammo ui. should make a separte event really
        ))
      (return _success)))
  (`self.AddNewWeapon` false _returnvalue)
  (return true))

(fn `SetupMaterial`
  (bind _mesh (`self.Mesh`))
  (bind _returnvalue (`PrimitiveComponent.CreateDynamicMaterialInstance` _mesh 0 (`PrimitiveComponent.GetMaterial` _mesh 0) "None"))
  (`MaterialInstanceDynamic.SetVectorParameterValue` _returnvalue "TeamColour" (`self.ArmourColour`))
  (`PrimitiveComponent.SetMaterial` _mesh 0 _returnvalue)
  (set `self.DynamicMaterial` _returnvalue))

(fn `TryFire`
  (if (and (not (`self.changingWeapons`)) (not (`self.dead`)))
    (bind _fired (`/Game/Framework_Blueprints/Weapons/Weapon_Base.CheckFire` (`|GetArrayItem` (`self.Weapons`) (`self.currentWeapon`))))
    (if _fired
      (`self.PlayFireAnim`))))

(fn `TryWeaponRefire`
  (if (`self.fireHeld`)
    (`self.TryFire`)))

(fn `UpdateWeaponActors`
  (bind _output (`|GetArrayItem` (`self.Weapons`) (`self.currentWeapon`)))
  (bind _output_2 (`|GetArrayItem` (`self.Weapons`) (`self.PreviousWeapon`)))
  (clear `/Game/Framework_Blueprints/Weapons/Weapon_Base.WeaponCooledDown` _output_2)
  (`self.K2_AttachToComponent` _output_2 (`self.Mesh`) "HolsterSocket" "SnapToTarget" "SnapToTarget" "KeepWorld" true)
  (add `/Game/Framework_Blueprints/Weapons/Weapon_Base.WeaponCooledDown` _output (`|CreateDelegate` :!event `TryWeaponRefire`))
  (`self.K2_AttachToComponent` _output (`self.Mesh`) "RightHandSocket" "SnapToTarget" "SnapToTarget" "KeepWorld" true))

(fn `UserConstructionScript`
  (bind _editordebugtext (`self.EditorDebugText`))
  (`self.SetupMaterial`)
  (`TextRenderComponent.K2_SetText` _editordebugtext (`self.DebugEditorText`))
  (`SceneComponent.SetAbsolute` _editordebugtext false true false))